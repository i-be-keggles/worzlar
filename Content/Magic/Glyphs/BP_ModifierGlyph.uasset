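; BP_ModifierGlyph is a spell glyph that modifies an action glyph and shares its lifetime, apparently serving as a base for modifier glyphs.
; ActivateOnActionGlyph stores the target action glyph and binds to its destroyed and deactivate events, either of which prints a debug message and destroys the modifier.
; Cast only forwards to the parent, and GetPhysicalRepresentation is an empty stub, so no modifier effect is implemented here.
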(event Custom|ActivateOnActionGlyph
  (params (ActionGlyph :type BP%20Action%20Glyph%20Object%20Reference))
  (bind _output_get (Variables|Default|SetTargetActionGlyph ActionGlyph))
  (Game|BindEventtoOnDestroyed _output_get (delegate Custom|Kill))
  (EventDispatchers|BindEventtoOnDeactivate _output_get (delegate Custom|Kill2)))

(event Custom|Kill
  (params (DestroyedActor :type Actor%20Object%20Reference))
  (Development|PrintString "Modifier deleting itself")
  (Actor|DestroyActor))

(event Custom|Kill2
  (Development|PrintString "Modifier deleting itself")
  (Actor|DestroyActor))

(event EventCast
  (params (Spell :type S%20Spell%20Structure) (Index :type Integer) (CastGlyphs :type Array%20of%20BP%20Glyph%20Object%20References) (Player :type BP%20First%20Person%20Character%20Object%20Reference))
  (|CallParentFunction Spell Index CastGlyphs Player))

(fn ConstructionScript
  (|CallParentFunction))

(fn GetPhysicalRepresentation
  (return 0))