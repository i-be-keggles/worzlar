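; Proximity trigger glyph for the spell system that fires when an actor comes within range.
; On Cast it runs the parent glyph logic, then scales its Sphere's world scale by Size.
; A begin overlap on the Sphere calls Trigger if the other actor has any ActorComponent, a check that filters very little.
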(event OnComponentBeginOverlap(Sphere)
  (params (OverlappedComponent :type Primitive%20Component%20Object%20Reference) (OtherActor :type Actor%20Object%20Reference) (OtherComp :type Primitive%20Component%20Object%20Reference) (OtherBodyIndex :type Integer) (bFromSweep :type Boolean) (SweepResult :type Hit%20Result%20Structure%20%28by%20ref%29))
  (Utilities|IsValid (Actor|GetComponentbyClass OtherActor "/Script/Engine.ActorComponent")
    (:Is%20Valid
      (CallFunction|Trigger))))

(event EventCast
  (params (Spell :type S%20Spell%20Structure) (Index :type Integer) (CastGlyphs :type Array%20of%20BP%20Glyph%20Object%20References) (Player :type BP%20Player%20Object%20Reference))
  (bind _sphere (Variables|Default|GetSphere))
  (|CallParentFunction Spell Index CastGlyphs Player)
  (Transformation|SetWorldScale3D _sphere (* (Transformation|GetWorldScale _sphere) (Variables|Default|GetSize))))

(fn ConstructionScript
  (|CallParentFunction))