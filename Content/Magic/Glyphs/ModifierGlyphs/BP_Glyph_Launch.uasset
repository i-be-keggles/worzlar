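; Modifier glyph in the magic glyph system that launches the physical form of the action glyph it modifies.
; On activation it runs the parent logic, then fetches the physical representation components from the target action glyph if that is valid.
; Each component gets physics simulation enabled and a single mass-independent AddForce along its own forward vector, scaled by Speed.
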(event EventActivateonActionGlyph
  (params (ActionGlyph :type BP%20Action%20Glyph%20Object%20Reference))
  (bind _targetactionglyph (Variables|Default|GetTargetActionGlyph))
  (|CallParentFunction ActionGlyph)
  (Utilities|IsValid _targetactionglyph
    (:Is%20Valid
      (bind _physical_components (Default|GetPhysicalRepresentation _targetactionglyph))
      (for _array_element _physical_components
        (Physics|SetSimulatePhysics _array_element true)
        (Physics|AddForce _array_element (* (Math|Vector|GetForwardVector _array_element) (Variables|Default|GetSpeed)) "None" true)))))

(fn ConstructionScript
  (|CallParentFunction))