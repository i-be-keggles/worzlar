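; Modifier glyph that makes an action glyph's physical representation home in on a nearby target.
; On activation it enables gravity-free physics on non-simulating parts and starts a looping FindTarget timer.
; FindTarget sphere-overlaps, ignoring the player, adds actors with BPC_Health to a never-cleared list and picks the nearest.
; Tick pushes parts toward the target; projectiles instead get force perpendicular to velocity plus turning torque.
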(event EventTick
  (params (DeltaSeconds :type Float%20%28single-precision%29))
  (bind _returnvalue (Transformation|GetActorLocation))
  (bind _targetactionglyph (Variables|Default|GetTargetActionGlyph))
  (bind _target (Variables|Default|GetTarget))
  (bind _rootcomponent (Variables|/Script/Engine.Actor|GetRootComponent _target))
  (bind _returnvalue_2 (Transformation|GetWorldLocation _rootcomponent))
  (bind _returnvalue_3 (- _returnvalue_2 _returnvalue))
  (bind _returnvalue_4 (Math|Vector|Normalize _returnvalue_3))
  (Utilities|IsValid _targetactionglyph
    (:Is%20Valid
      (Utilities|IsValid (Variables|Default|GetTarget)
        (:Is%20Valid
          (bind _physical_components (Default|GetPhysicalRepresentation _targetactionglyph))
          (for _array_element _physical_components
            (if (Variables|Default|GetRotate)
              (Physics|AddForce _array_element (* (Variables|Default|GetSpeed) (- _returnvalue_4 (* (Math|Vector|DotProduct _returnvalue_4 (Math|Vector|Normalize (Transformation|GetComponentVelocity _array_element))) (Math|Vector|Normalize (Transformation|GetComponentVelocity _array_element)))) (Math|Conversions|ToVector(Float) 2.0)) "None" true)
              (Class|PrimitiveComponent|AddTorqueinDegrees _array_element (* (Math|Vector|CrossProduct (Math|Vector|GetForwardVector _array_element) _returnvalue_4) (Variables|Default|GetSpeed) (Math|Conversions|ToVector(Float) 0.3)) "None" true)
              (else
                (Physics|AddForce _array_element (* (Variables|Default|GetSpeed) _returnvalue_4) "None" true)))))))))

(event EventActivateonActionGlyph
  (params (ActionGlyph :type BP%20Action%20Glyph%20Object%20Reference))
  (bind _targetactionglyph (Variables|Default|GetTargetActionGlyph))
  (|CallParentFunction ActionGlyph)
  (Utilities|IsValid _targetactionglyph
    (:Is%20Valid
      (bind _physical_components (Default|GetPhysicalRepresentation _targetactionglyph))
      (Variables|Default|SetRotate (Utilities|IsValid (Actor|GetComponentbyClass _targetactionglyph "/Game/Util/FunctionalComponents/BPC_Projectile.BPC_Projectile_C")))
      (for _array_element _physical_components
        (if (not (Physics|IsSimulatingPhysics _array_element "None"))
          (Physics|SetSimulatePhysics _array_element true)
          (Physics|SetEnableGravity _array_element false)))
      (Utilities|Time|SetTimerbyFunctionName 0 "FindTarget" 0.3 true))))

(fn ConstructionScript
  (|CallParentFunction))

(fn FindTarget
  ;[1 1 1] TODO: filter by gameplay tags
  (bind (_outactors _returnvalue) (Collision|SphereOverlapActors (Transformation|GetActorLocation) (Variables|Default|GetSize) (Utilities|Array|MakeArray "ObjectTypeQuery1" "ObjectTypeQuery2" "ObjectTypeQuery3" "ObjectTypeQuery4") 0 (Utilities|Array|MakeArray (Game|Player|GetPlayerPawn 0))))
  (if _returnvalue
    (Utilities|FlowControl|Sequence
      (:then_0
        (for _array_element _outactors
          (Utilities|IsValid (Actor|GetComponentbyClass _array_element "/Game/Util/FunctionalComponents/BPC_Health.BPC_Health_C")
            (:Is%20Valid
              (Utilities|Array|Add (LocalVariables|GetTargets) _array_element))))
        (if (Utilities|Array|IsEmpty (LocalVariables|GetTargets))
          (return)))
      (:then_1
        (bind _output_get (Variables|Default|SetTarget (Utilities|Array|Get(acopy) (LocalVariables|GetTargets))))
        (Variables|Default|SetCachedDistance (Math|Vector|Distance(Vector) (Transformation|GetWorldLocation (Variables|/Script/Engine.Actor|GetRootComponent _output_get)) (Transformation|GetActorLocation))))
      (:then_2
        (for _array_element_2 (LocalVariables|GetTargets)
          (if (< (Math|Vector|Distance(Vector) (Transformation|GetWorldLocation (Variables|/Script/Engine.Actor|GetRootComponent _array_element_2)) (Transformation|GetActorLocation)) (Variables|Default|GetCachedDistance))
            (Variables|Default|SetCachedDistance (Math|Vector|Distance(Vector) (Transformation|GetWorldLocation (Variables|/Script/Engine.Actor|GetRootComponent _array_element_2)) (Transformation|GetActorLocation)))
            (Variables|Default|SetTarget _array_element_2)))))))