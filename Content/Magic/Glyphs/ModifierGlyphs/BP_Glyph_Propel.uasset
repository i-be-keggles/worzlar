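; BP_Glyph_Propel is a modifier glyph in the magic system that propels the physical representation of the action glyph it modifies.
; On activation it calls the parent logic, then enables physics simulation on each component of that glyph's physical representation.
; Every tick, while the target action glyph is valid, it pushes each component along its own forward vector with a mass-independent force scaled by Force.
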(event EventTick
  (params (DeltaSeconds :type Float%20%28single-precision%29))
  (bind _targetactionglyph (Variables|Default|GetTargetActionGlyph))
  (Utilities|IsValid _targetactionglyph
    (:Is%20Valid
      (bind _physical_components (Default|GetPhysicalRepresentation _targetactionglyph))
      (for _array_element _physical_components
        (Physics|AddForce _array_element (* (Math|Vector|GetForwardVector _array_element) (Variables|Default|GetForce)) "None" true)))))

(event EventActivateonActionGlyph
  (params (ActionGlyph :type BP%20Action%20Glyph%20Object%20Reference))
  (|CallParentFunction ActionGlyph)
  (bind _physical_components (Default|GetPhysicalRepresentation (Variables|Default|GetTargetActionGlyph)))
  (for _array_element _physical_components
    (Physics|SetSimulatePhysics _array_element true)))

(fn ConstructionScript
  (|CallParentFunction))