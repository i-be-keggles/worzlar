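; BP_Glyph is a glyph in the magic system, apparently a base for specific glyphs.
; Its Cast event stores the spell, its index, the cast glyphs and the player.
; If a particle template is valid, Cast spawns that Niagara system attached to the root, keeps the reference and sets it to the root's world location.
; GetPhysicalRepresentation returns nothing here, and the construction script is empty.
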(event Custom|Cast
  (params (Spell :type S%20Spell%20Structure) (Index :type Integer) (CastGlyphs :type Array%20of%20BP%20Glyph%20Object%20References) (Player :type BP%20First%20Person%20Character%20Object%20Reference))
  (bind _defaultsceneroot (Variables|Default|GetDefaultSceneRoot))
  (bind _returnvalue (Transformation|GetWorldLocation _defaultsceneroot))
  (Variables|Default|SetSpell Spell)
  (Variables|Default|SetIndex Index)
  (Variables|Default|SetPlayer Player)
  (Variables|Default|SetCast%20Glyphs CastGlyphs)
  (Utilities|IsValid (Variables|Default|GetParticleTemplate)
    (:Is%20Valid
      (bind _returnvalue_2 (Niagara|SpawnSystemAttached (Variables|Default|GetParticleTemplate) (Variables|Default|GetDefaultSceneRoot) "None" _returnvalue "0, 0, 0" "SnapToTarget" false))
      (bind _output_get (Variables|Default|SetParticles _returnvalue_2))
      (Transformation|SetWorldLocation _output_get _returnvalue false false))))

(fn ConstructionScript)

(fn GetPhysicalRepresentation
  (return 0))