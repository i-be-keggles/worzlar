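; Action glyph for the spell system that casts a fireball projectile, which explodes when it hits.
; Cast starts looping whoosh audio, binds the projectile component's hit event, sets the sphere to ignore all collision, and arms after a short delay.
; An armed hit spawns BP_Explosion using the glyph's damage and scaled size, then terminates; lifetime expiry also terminates.
; Termination stops effects, audio and movement, then destroys the actor after a delay.
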(event OnComponentHit(Sphere)
  (params (HitComponent :type Primitive%20Component%20Object%20Reference) (OtherActor :type Actor%20Object%20Reference) (OtherComp :type Primitive%20Component%20Object%20Reference) (NormalImpulse :type Vector :default "0, 0, 0") (Hit :type Hit%20Result%20Structure%20%28by%20ref%29)))

(event Custom|ProjectileHit
  (params (Hit :type Actor%20Object%20Reference))
  (if (Variables|Default|GetActive)
    (bind _returnvalue (Game|SpawnActorfromClass "/Game/Util/FunctionalComponents/BP_Explosion.BP_Explosion_C" (Math|Transform|MakeTransform (Transformation|GetWorldLocation (Variables|Default|GetSphere)) "0, 0, 0" "1.000000,1.000000,1.000000") "Undefined" "MultiplyWithRoot" 0 0))
    (Default|Explode _returnvalue (Variables|Default|GetDamage) (* (Variables|Default|GetSize) 5.0) "/Game/VFX/NS_FireBurst.NS_FireBurst" "/Game/SFX/WaveAssets/Magic/FireBallExplosion.FireBallExplosion")
    (Default|CallOnTerminate)))

(event EventHandleTerminate
  (bind _bpc_projectile (Variables|Default|GetBPC_Projectile))
  (Components|Activation|Deactivate (Variables|Default|GetParticles))
  (Utilities|FlowControl|Sequence
    (:then_0
      (Audio|Components|Audio|Stop (Variables|Default|GetAudio))
      (Utilities|IsValid _bpc_projectile
        (:Is%20Valid
          (Components|DestroyComponent _bpc_projectile))))
    (:then_1
      (CallFunction|Deactivate)
      (Physics|SetSimulatePhysics (Variables|Default|GetSphere) false)
      (Utilities|FlowControl|Delay 3.0)
      (Actor|DestroyActor))))

(event EventCast
  (params (Spell :type S%20Spell%20Structure) (Index :type Integer) (CastGlyphs :type Array%20of%20BP%20Glyph%20Object%20References) (Player :type BP%20Player%20Object%20Reference))
  (bind _audio (Variables|Default|GetAudio))
  (|CallParentFunction Spell Index CastGlyphs Player)
  (Utilities|FlowControl|Sequence
    (:then_0
      (Class|AudioComponent|SetWaveParameter _audio "Sound" "/Game/SFX/WaveAssets/Magic/FireballWhoosh.FireballWhoosh")
      (Audio|Components|Audio|Play _audio 0.0)
      (Effects|Components|ParticleSystem|SetBoolParameter _audio "Loop" true)
      (EventDispatchers|BindEventtoOnProjectileHit (Variables|Default|GetBPC_Projectile) (delegate Custom|ProjectileHit)))
    (:then_1
      (Collision|SetCollisionResponsetoAllChannels (Variables|Default|GetSphere) "ECR_Ignore")
      (Utilities|FlowControl|Delay 0.2)
      (Variables|Default|SetActive true)
      (Utilities|FlowControl|Delay (Variables|Default|GetLifetime))
      (Default|CallOnTerminate))))

(fn ConstructionScript
  (|CallParentFunction))

(fn GetPhysicalRepresentation
  (return (Utilities|Array|MakeArray (Variables|Default|GetSphere))))