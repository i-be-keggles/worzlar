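; Blink action glyph that teleports the casting player forward along the glyph's facing direction.
; On cast it runs the parent logic, plays a whoosh through a MetaSound wave parameter, and line-traces forward by the glyph's Size, ignoring the player.
; The player lands at the hit point or the trace end without sweeping, then the glyph terminates.
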(event EventCast
  (params (Spell :type S%20Spell%20Structure) (Index :type Integer) (CastGlyphs :type Array%20of%20BP%20Glyph%20Object%20References) (Player :type BP%20Player%20Object%20Reference))
  (bind _returnvalue (Transformation|GetActorLocation))
  (|CallParentFunction Spell Index CastGlyphs Player)
  (bind _returnvalue_2 (Audio|SpawnSoundatLocation "/Game/SFX/Metasounds/MS_BasicSound.MS_BasicSound" (Transformation|GetActorLocation) "0, 0, 0" 2.0 1.0 0.0 0 0))
  (Class|AudioComponent|SetWaveParameter _returnvalue_2 "Sound" "/Game/SFX/WaveAssets/Magic/BlinkWhoosh.BlinkWhoosh")
  (bind (_outhit _returnvalue_3) (Collision|LineTraceByChannel _returnvalue (+ _returnvalue (* (Transformation|GetActorForwardVector) (Variables|Default|GetSize))) "TraceTypeQuery1" false (Utilities|Array|MakeArray (Variables|Default|GetPlayer)) "None"))
  (Transformation|SetActorLocation (Variables|Default|GetPlayer) (Math|Vector|SelectVector (.location _outhit) (.traceend _outhit) _returnvalue_3) false true)
  (CallFunction|Terminate))

(fn ConstructionScript
  (|CallParentFunction))

(fn GetPhysicalRepresentation
  (return (Utilities|Array|MakeArray 0)))