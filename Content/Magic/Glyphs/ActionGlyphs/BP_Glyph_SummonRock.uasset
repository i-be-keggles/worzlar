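; Action glyph for the magic system that summons a physical rock as its spell effect.
; On cast it nudges the mesh forward, scales it by Size, and terminates after Lifetime, with actor destruction following a short delay after termination.
; Hard impacts play a rock sound through a MetaSound, gated by an impulse threshold and brief cooldown.
; The mesh is exposed as the glyph's physical representation.
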(event OnComponentHit(StaticMesh)
  (params (HitComponent :type Primitive%20Component%20Object%20Reference) (OtherActor :type Actor%20Object%20Reference) (OtherComp :type Primitive%20Component%20Object%20Reference) (NormalImpulse :type Vector :default "0, 0, 0") (Hit :type Hit%20Result%20Structure%20%28by%20ref%29))
  (if (Variables|Default|GetCanMakeSound)
    (if (> (Math|Vector|VectorLength NormalImpulse) 1.5e+04)
      (Utilities|FlowControl|Sequence
        (:then_0
          (bind _returnvalue (Audio|SpawnSoundatLocation "/Game/SFX/Metasounds/MS_BasicSound.MS_BasicSound" (Transformation|GetWorldLocation (Variables|Default|GetStaticMesh)) "0, 0, 0" 1.0 1.0 0.0 "/Game/SFX/Attenuation/AS_AttenuationMedium.AS_AttenuationMedium" 0))
          (Class|AudioComponent|SetWaveParameter _returnvalue "Sound" "/Game/SFX/WaveAssets/Impacts/RockImpact.RockImpact"))
        (:then_1
          (Variables|Default|SetCanMakeSound false)
          (Utilities|FlowControl|Delay 0.2)
          (Variables|Default|SetCanMakeSound true))))))

(event EventHandleTerminate
  (Utilities|FlowControl|Delay 3.0)
  (Actor|DestroyActor))

(event EventCast
  (params (Spell :type S%20Spell%20Structure) (Index :type Integer) (CastGlyphs :type Array%20of%20BP%20Glyph%20Object%20References) (Player :type BP%20Player%20Object%20Reference))
  (bind _staticmesh (Variables|Default|GetStaticMesh))
  (|CallParentFunction Spell Index CastGlyphs Player)
  (Transformation|SetWorldLocation _staticmesh (+ (Transformation|GetWorldLocation _staticmesh) (* (Math|Vector|GetForwardVector _staticmesh) (Math|Conversions|ToVector(Float) 5e+01))) false false)
  (Transformation|SetWorldScale3D (Variables|Default|GetStaticMesh) (Math|Conversions|ToVector(Float) (Variables|Default|GetSize)))
  (Utilities|FlowControl|Delay (Variables|Default|GetLifetime))
  (CallFunction|Terminate))

(fn ConstructionScript
  (|CallParentFunction))

(fn GetPhysicalRepresentation
  (return (Utilities|Array|MakeArray (Variables|Default|GetStaticMesh))))