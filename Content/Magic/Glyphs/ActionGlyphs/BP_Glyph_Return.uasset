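; BP_Glyph_Return is an action glyph in the spell system that teleports the casting player to the glyph actor's location.
; On Cast it runs the parent logic, plays a blink whoosh at that location by feeding the wave into a generic MetaSound parameter, moves the player without sweeping, then terminates.
; It also overrides GetPhysicalRepresentation, while its construction script only calls the parent.
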(event EventCast
  (params (Spell :type S%20Spell%20Structure) (Index :type Integer) (CastGlyphs :type Array%20of%20BP%20Glyph%20Object%20References) (Player :type BP%20Player%20Object%20Reference))
  (bind _returnvalue (Transformation|GetActorLocation))
  (|CallParentFunction Spell Index CastGlyphs Player)
  (bind _returnvalue_2 (Audio|SpawnSoundatLocation "/Game/SFX/Metasounds/MS_BasicSound.MS_BasicSound" _returnvalue "0, 0, 0" 2.0 1.0 0.0 0 0))
  (Class|AudioComponent|SetWaveParameter _returnvalue_2 "Sound" "/Game/SFX/WaveAssets/Magic/BlinkWhoosh.BlinkWhoosh")
  (Transformation|SetActorLocation (Variables|Default|GetPlayer) _returnvalue false true)
  (CallFunction|Terminate))

(fn ConstructionScript
  (|CallParentFunction))

(fn GetPhysicalRepresentation
  (return (Utilities|Array|MakeArray 0)))