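; BP_Glyph_ArcaneBolt is an action glyph for a projectile spell that deals elemental damage on impact.
; Casting plays a whoosh, binds to the projectile component's hit event and starts a lifetime timer.
; A hit terminates the bolt, sends damage to the target's health component and spawns a burst effect.
; Termination stops particles, removes the projectile component, plays a hiss and delays actor destruction so effects finish.
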(event Custom|OnCollision
  (params (Hit :type Actor%20Object%20Reference))
  (CallFunction|Terminate)
  (Class|BPIHealth|TakeDamage(Message) (Actor|GetComponentbyClass Hit "/Game/Util/FunctionalComponents/BPC_Health.BPC_Health_C") (Math|Float|Truncate (Variables|Default|GetDamage)) (Variables|Default|GetElementType) self)
  (Niagara|SpawnSystematLocation "/Game/VFX/NS_MagicBurstTiny.NS_MagicBurstTiny" (Transformation|GetWorldLocation (Variables|Default|GetSphere)) "0, 0, 0" (Math|Conversions|ToVector(Float) 1.0)))

(event EventHandleTerminate
  (bind _bpc_projectile (Variables|Default|GetBPC_Projectile))
  (Utilities|FlowControl|Sequence
    (:then_0
      (Components|Activation|Deactivate (Variables|Default|GetParticles))
      (Utilities|IsValid _bpc_projectile
        (:Is%20Valid
          (Components|DestroyComponent _bpc_projectile))))
    (:then_1
      (bind _returnvalue (Audio|SpawnSoundatLocation "/Game/SFX/Magic/MS_BasicSound.MS_BasicSound" (Transformation|GetWorldLocation (Variables|Default|GetSphere)) "0, 0, 0" 1.0 1.0 0.0 "/Game/SFX/Attenuation/AS_AttenuationMedium.AS_AttenuationMedium" 0))
      (Class|AudioComponent|SetWaveParameter _returnvalue "Sound" "/Game/SFX/Impacts/SmallMagicHiss.SmallMagicHiss"))
    (:then_2
      (Utilities|FlowControl|Delay 3.0)
      (Actor|DestroyActor))))

(event EventCast
  (params (Spell :type S%20Spell%20Structure) (Index :type Integer) (CastGlyphs :type Array%20of%20BP%20Glyph%20Object%20References) (Player :type BP%20Player%20Object%20Reference))
  (bind _audio (Variables|Default|GetAudio))
  (|CallParentFunction Spell Index CastGlyphs Player)
  (Utilities|FlowControl|Sequence
    (:then_0
      (Class|AudioComponent|SetWaveParameter _audio "Sound" "/Game/SFX/Magic/BlinkWhoosh.BlinkWhoosh")
      (Audio|Components|Audio|Play _audio 0.0)
      (EventDispatchers|BindEventtoOnProjectileHit (Variables|Default|GetBPC_Projectile) (delegate Custom|OnCollision)))
    (:then_1
      (Utilities|FlowControl|Delay (Variables|Default|GetLifetime))
      (CallFunction|Terminate))))

(fn ConstructionScript
  (|CallParentFunction))

(fn GetPhysicalRepresentation
  (return (Utilities|Array|MakeArray (Variables|Default|GetSphere))))