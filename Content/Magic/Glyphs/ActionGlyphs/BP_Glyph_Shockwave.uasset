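; Action glyph for the magic system that releases a shockwave explosion when cast.
; On Cast it runs the parent logic, spawns a BP_Explosion at its own transform and triggers it with the glyph's Size as radius plus shockwave particles and sound.
; It then destroys itself and calls Terminate; its Damage variable is unused.
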(event EventCast
  (params (Spell :type S%20Spell%20Structure) (Index :type Integer) (CastGlyphs :type Array%20of%20BP%20Glyph%20Object%20References) (Player :type BP%20Player%20Object%20Reference))
  (|CallParentFunction Spell Index CastGlyphs Player)
  (bind _returnvalue (Game|SpawnActorfromClass "/Game/Util/FunctionalComponents/BP_Explosion.BP_Explosion_C" (Transformation|GetActorTransform) "Undefined" "MultiplyWithRoot" 0 0))
  (Default|Explode _returnvalue 0.0 (Variables|Default|GetSize) 0.0 "/Game/VFX/NiagaraSystems/NS_Shockwave.NS_Shockwave" "/Game/SFX/WaveAssets/Magic/Shockwave.Shockwave")
  (Actor|DestroyActor)
  (CallFunction|Terminate))

(fn ConstructionScript
  (|CallParentFunction))

(fn GetPhysicalRepresentation
  (return (Utilities|Array|MakeArray 0)))