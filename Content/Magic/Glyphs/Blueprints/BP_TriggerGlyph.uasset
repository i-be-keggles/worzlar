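; BP_TriggerGlyph is a spell glyph that resumes casting of its spell from a stored index when triggered.
; On Cast it searches earlier cast glyphs for an action glyph, attaches to that glyph's physical representation and records it as the previous action.
; SetupTrigger supplies the return index and sibling triggers; Trigger has the Player continue the spell with itself as caster, then terminates the siblings and itself.
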(event Custom|Trigger
  (Default|CastSpell (Variables|Default|GetPlayer) (Variables|Default|GetSpell) (Variables|Default|GetReturn%20to%20Index) self)
  (for _array_element (Variables|Default|GetOther%20Triggers)
    (Default|Terminate _array_element))
  (CallFunction|Terminate))

(event Custom|SetupTrigger
  (params (ReturnToIndex :type Integer) (OtherTriggers :type Array%20of%20BP%20Trigger%20Glyph%20Object%20References))
  (Variables|Default|SetReturn%20to%20Index ReturnToIndex)
  (Variables|Default|SetOther%20Triggers OtherTriggers))

(event EventHandleTerminate
  (Actor|DestroyActor))

(event EventCast
  (params (Spell :type S%20Spell%20Structure) (Index :type Integer) (CastGlyphs :type Array%20of%20BP%20Glyph%20Object%20References) (Player :type BP%20Player%20Object%20Reference))
  (|CallParentFunction Spell Index CastGlyphs Player)
  ;[1 1 1] Attach to prev action
  (bind _index (Utilities|FlowControl|ForLoopwithBreak 1 Index :!label _label)
    (:LoopBody
      (Utilities|IsValid (Utilities|Array|Get(acopy) CastGlyphs (- Index _index))
        (:Is%20Valid
          (bind _asbp_action_glyph (Utilities|Casting|CastToBP_ActionGlyph (Utilities|Array|Get(acopy) CastGlyphs (- Index _index))))
          (bind _physical_components (Default|GetPhysicalRepresentation _asbp_action_glyph))
          (Utilities|FlowControl|Sequence
            (:then_0
              (Utilities|IsValid (Utilities|Array|Get(acopy) _physical_components)
                (:Is%20Valid
                  (Transformation|AttachComponentToComponent (Utilities|Array|Get(acopy) _physical_components) "None" "SnapToTarget" "SnapToTarget" "KeepWorld" true))))
            (:then_1
              (Variables|Default|SetPrevActionGlyph _asbp_action_glyph))
            (:then_2
              (goto _label Break))))))))

(fn ConstructionScript
  (|CallParentFunction))

(fn GetPhysicalRepresentation
  (return 0))