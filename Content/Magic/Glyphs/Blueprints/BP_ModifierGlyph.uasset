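; BP_ModifierGlyph is a spell glyph that modifies an action glyph, with casting deferred to its parent class.
; On activation it stores the target action glyph and snaps to its root component, keeping world scale.
; It binds to the target's terminate event to end alongside it, destroying itself when termination is handled.
; It returns no physical representation of its own.
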(event Custom|ActivateOnActionGlyph
  (params (ActionGlyph :type BP%20Action%20Glyph%20Object%20Reference))
  (bind _output_get (Variables|Default|SetTargetActionGlyph ActionGlyph))
  (Transformation|AttachComponentToComponent (Variables|/Script/Engine.Actor|GetRootComponent _output_get) "None" "SnapToTarget" "SnapToTarget" "KeepWorld" true)
  (EventDispatchers|BindEventtoOnTerminate _output_get (delegate Custom|ModifierTerminatePassthrough)))

(event Custom|ModifierTerminatePassthrough
  (CallFunction|Terminate))

(event EventHandleTerminate
  (Actor|DestroyActor))

(event EventCast
  (params (Spell :type S%20Spell%20Structure) (Index :type Integer) (CastGlyphs :type Array%20of%20BP%20Glyph%20Object%20References) (Player :type BP%20Player%20Object%20Reference))
  (|CallParentFunction Spell Index CastGlyphs Player))

(fn ConstructionScript
  (|CallParentFunction))

(fn GetPhysicalRepresentation
  (return 0))