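; BP_ActionGlyph is a base action glyph in the spell system, with an overridable physical representation that is empty here.
; On Cast, it runs the parent cast, then attaches its particles to that representation.
; It then walks back through the preceding cast glyphs, activating each consecutive modifier glyph on itself until it reaches a non-modifier.
; Deactivate clears the active flag and fires an on-deactivate notification.
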(event Custom|Deactivate
  (Variables|Default|SetActive false)
  (Default|CallOnDeactivate))

(event EventCast
  (params (Spell :type S%20Spell%20Structure) (Index :type Integer) (CastGlyphs :type Array%20of%20BP%20Glyph%20Object%20References) (Player :type BP%20First%20Person%20Character%20Object%20Reference))
  (|CallParentFunction Spell Index CastGlyphs Player)
  (Utilities|FlowControl|Sequence
    (:then_0
      ;[1 1 1] Attach particles
      (bind _physical_components (CallFunction|GetPhysicalRepresentation))
      (Transformation|AttachComponentToComponent (Variables|Default|GetParticles) (Utilities|Array|Get(acopy) _physical_components) "None" "KeepRelative" "KeepRelative" "KeepRelative" true))
    (:then_1
      ;[1 1 1] Activate modifiers
      (bind _index (Utilities|FlowControl|ForLoopwithBreak 1 Index :!label _label)
        (:LoopBody
          (bind _asbp_modifier_glyph (Utilities|Casting|CastToBP_ModifierGlyph (Utilities|Array|Get(acopy) CastGlyphs (- Index _index)))
            (:then
              (Default|ActivateonActionGlyph _asbp_modifier_glyph self))
            (:CastFailed
              (goto _label Break))))))))

(fn ConstructionScript
  (|CallParentFunction))

(fn GetPhysicalRepresentation
  (return 0))