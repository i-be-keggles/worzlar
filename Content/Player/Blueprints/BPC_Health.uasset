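; BPC_Health is a health component for the player that tracks damage and death.
; Health starts at MaxHealth on BeginPlay, and TakeDamage subtracts the amount, clamped at zero.
; At zero health it calls Die, which prints a debug message and broadcasts OnDied.
; Every hit then broadcasts OnTookDamage and a passthrough dispatcher carrying amount, type and source.
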(event EventBeginPlay
  (Variables|Default|SetHealth (Variables|Default|GetMaxHealth)))

(event EventTick
  (params (DeltaSeconds :type Float%20%28single-precision%29)))

(event EventTakeDamage
  (params (Amount :type Integer) (Type :type E_ElementType%20Enum :default "NewEnumerator0") (Source :type Actor%20Object%20Reference))
  (bind _output_get (Variables|Default|SetHealth (Math|Integer|Max(Integer) (- (Variables|Default|GetHealth) Amount))))
  (Utilities|FlowControl|Sequence
    (:then_0
      (if (<= _output_get 0)
        (CallFunction|Die)))
    (:then_1
      (Default|CallOnTookDamage)
      (Default|CallOnTookDamagePassthrough Amount Type Source))))

(event EventDie
  (Development|PrintString "Died")
  (Default|CallOnDied))