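; Player dash component that launches the owning character on the dash input, with a cooldown.
; Cached move input picks the direction: backward takes priority, then sideways, otherwise forward along the actor's axes.
; Each dash temporarily overrides falling lateral friction, restoring it after a short delay, and plays a whoosh sound.
; It triggers the cooldown display on the player's HUD, cached shortly after BeginPlay, and leaves debug prints in place.
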(event Input|EnhancedActionEvents|EnhancedInputActionIA_Dash
  (params (ActionValue :type Boolean) (ElapsedSeconds :type Float%20%28double-precision%29) (TriggeredSeconds :type Float%20%28double-precision%29) (InputAction :type Input%20Action%20Object%20Reference :default "/Game/Player/Input/Actions/IA_Dash.IA_Dash"))
  (bind _inputdir (Variables|Default|GetInputDir))
  (bind _hud (Variables|Default|GetHUD))
  (bind _character (Variables|Default|GetCharacter))
  (bind _character_2 (Variables|Default|GetCharacter))
  (bind _speed (Variables|Default|GetSpeed))
  (bind _returnvalue (Transformation|GetActorForwardVector _character))
  (bind (_x _y) (Math|Vector2D|BreakVector2D _inputdir))
  (bind _charactermovement (Variables|/Script/Engine.Character|GetCharacterMovement _character_2))
  (bind _returnvalue_2 (* _returnvalue _speed))
  (if ActionValue
    (if (Variables|Default|GetCanDash)
      (Utilities|FlowControl|Sequence
        (:then_0
          (Variables|Default|SetPrevFriction (Variables|/Script/Engine.CharacterMovementComponent|GetFallingLateralFriction _charactermovement))
          (Variables|/Script/Engine.CharacterMovementComponent|SetFallingLateralFriction _charactermovement 3.0))
        (:then_1
          (Variables|Default|SetPrevVel (Transformation|GetVelocity (Variables|Default|GetCharacter)))
          (if (< _y 0.0)
            (Character|LaunchCharacter _character (* (Math|Conversions|ToVector(Float) -1.0) _returnvalue_2) false false)
            (elif (!= _x 0.0)
              (Character|LaunchCharacter _character (* (Math|Float|SelectFloat 1.0 -1.0 (> _x 0.0)) (Transformation|GetActorRightVector _character) (Variables|Default|GetSpeed)) false false)
              (else
                (Character|LaunchCharacter _character _returnvalue_2 false false)))))
        (:then_2
          (Audio|PlaySound2D "/Game/SFX/WaveAssets/Magic/DashWoosh.DashWoosh" 0.5 1.0 0.0 0 0))
        (:then_3
          (Utilities|IsValid _hud
            (:Is%20Valid
              (Default|TriggerDashCooldown _hud (Variables|Default|GetCooldown))
              (Development|PrintString "Yoped"))
            (:Is%20Not%20Valid
              (Development|PrintString "Noped"))))
        (:then_4
          (Utilities|FlowControl|Delay 0.8)
          (Variables|/Script/Engine.CharacterMovementComponent|SetFallingLateralFriction _charactermovement (Variables|Default|GetPrevFriction)))
        (:then_5
          (Variables|Default|SetCanDash false)
          (Utilities|FlowControl|Delay (Variables|Default|GetCooldown))
          (Variables|Default|SetCanDash true))))))

(event Input|EnhancedActionEvents|EnhancedInputActionIA_Move
  (params (ActionValue :type Vector%202D%20Structure) (ElapsedSeconds :type Float%20%28double-precision%29) (TriggeredSeconds :type Float%20%28double-precision%29) (InputAction :type Input%20Action%20Object%20Reference :default "/Game/Player/Input/Actions/IA_Move.IA_Move"))
  (:Triggered
    (Variables|Default|SetInputDir ActionValue))
  (:Canceled
    (Variables|Default|SetInputDir "" :!label _label))
  (:Completed
    (goto _label)))

(event EventBeginPlay
  (bind _returnvalue (Components|GetOwner))
  (bind _ascharacter (Utilities|Casting|CastToCharacter _returnvalue))
  (Variables|Default|SetCharacter _ascharacter)
  (bind _asbp_player (Utilities|Casting|CastToBP_Player _returnvalue))
  (Utilities|FlowControl|Delay 0.2)
  (Variables|Default|SetHUD (Variables|/Game/Player/Blueprints/BP_Player.BP_Player_C|GetHUD _asbp_player)))