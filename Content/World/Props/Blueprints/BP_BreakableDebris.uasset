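; Breakable debris prop that shatters when its health component dies, including from hard physics impacts.
; A static mesh hit with a normal impulse above a threshold sends a die message to BPC_Health.
; On death it plays an attenuated MetaSound, injecting the plate shatter wave as a parameter, spawns the pot-break Niagara effect at the mesh, and destroys itself.
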(event OnDied(BPC_Health)
  (bind _staticmesh (Variables|Default|GetStaticMesh))
  (bind _returnvalue (Transformation|GetWorldLocation _staticmesh))
  (bind _returnvalue_2 (Audio|SpawnSoundatLocation "/Game/SFX/Metasounds/MS_BasicVariation.MS_BasicVariation" _returnvalue "0, 0, 0" 1.0 1.0 0.0 "/Game/SFX/Attenuation/AS_AttenuationMedium.AS_AttenuationMedium" 0))
  (Class|AudioComponent|SetWaveParameter _returnvalue_2 "Sound" "/Game/SFX/WaveAssets/Impacts/PlateShatter.PlateShatter")
  (Niagara|SpawnSystematLocation "/Game/VFX/NiagaraSystems/NS_BreakPot.NS_BreakPot" _returnvalue)
  (Actor|DestroyActor))

(event OnComponentHit(StaticMesh)
  (params (HitComponent :type Primitive%20Component%20Object%20Reference) (OtherActor :type Actor%20Object%20Reference) (OtherComp :type Primitive%20Component%20Object%20Reference) (NormalImpulse :type Vector :default "0, 0, 0") (Hit :type Hit%20Result%20Structure%20%28by%20ref%29))
  (if (> (Math|Vector|VectorLength NormalImpulse) 3e+04)
    (Class|BPIHealth|Die(Message) (Variables|Default|GetBPC_Health))))

(event EventBeginPlay)

(event Collision|EventActorBeginOverlap
  (params (OtherActor :type Actor%20Object%20Reference)))

(event EventTick
  (params (DeltaSeconds :type Float%20%28single-precision%29)))

(fn ConstructionScript)