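; BPC_StatusEffect is a base actor component for timed status effects, with empty activation, tick and termination events for subclasses to override.
; StartEffect runs activation and starts two looping timers, one for ticks and one counting down Lifetime in half-second steps.
; ApplyAgain either adds to or takes the maximum Lifetime, per TimeStacks, then reruns activation.
; The owner receives applied and ended messages, and the component destroys itself on expiry.
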(event Custom|StartEffect
  (CallFunction|ActivationBehaviour)
  (Utilities|Time|SetTimerbyEvent (delegate Custom|TickBehaviour) (Variables|Default|GetTickSpeed) true)
  (Utilities|Time|SetTimerbyEvent (delegate Custom|LifetimeTickdown) (Math|Float|MakeLiteralFloat 0.5) true)
  (bind _output_get (Variables|Default|SetOwningActor (Components|GetOwner)))
  (Class|BPIStatusReactiveActor|OnStatusApplied(Message) _output_get self))

(event Custom|EndEffect
  (CallFunction|TerminationBehaviour)
  (Class|BPIStatusReactiveActor|OnStatusEnded(Message) (Variables|Default|GetOwningActor) (Utilities|GetClass self))
  (Components|DestroyComponent))

(event Custom|ActivationBehaviour
  ;[1 1 1] Override in subclass for logic
)

(event Custom|TickBehaviour
  ;[1 1 1] Override in subclass for logic
)

(event Custom|LifetimeTickdown
  (bind _output_get (Variables|Default|SetLifetime (- (Variables|Default|GetLifetime) (Math|Float|MakeLiteralFloat 0.5))))
  (if (<= _output_get 0.0)
    (CallFunction|EndEffect)))

(event Custom|TerminationBehaviour
  ;[1 1 1] Override in subclass for logic
)

(event Custom|ApplyAgain
  (params (Lifetime :type Float%20%28double-precision%29))
  (Utilities|FlowControl|Sequence
    (:then_0
      (if (Variables|Default|GetTimeStacks)
        (Variables|Default|SetLifetime (+ (Variables|Default|GetLifetime) Lifetime))
        (else
          (Variables|Default|SetLifetime (Math|Float|Max(Float) (Variables|Default|GetLifetime) Lifetime)))))
    (:then_1
      (CallFunction|ActivationBehaviour)
      (Class|BPIStatusReactiveActor|OnStatusApplied(Message) (Variables|Default|GetOwningActor) self))))