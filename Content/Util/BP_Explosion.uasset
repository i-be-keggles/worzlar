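; BP_Explosion is a utility actor that produces a one-shot explosion with damage and knockback when Explode is called.
; Explode spawns the supplied particle system and plays a fireball sound, then after a brief delay runs a radius sphere overlap.
; Overlapped actors with BPC_Health take damage, physics-simulating roots get an outward force scaled by radius over distance, and each name is debug-printed.
; The actor destroys itself seconds later.
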(event Custom|Explode
  (params (Damage :type Float%20%28double-precision%29) (Radius :type Float%20%28double-precision%29) (Particles :type Niagara%20System%20Object%20Reference))
  (bind _ms_fireballexplosion (Variables|Default|GetMS_FireballExplosion))
  (Utilities|FlowControl|Sequence
    (:then_0
      (Niagara|SpawnSystematLocation Particles (Transformation|GetWorldLocation (Variables|Default|GetDefaultSceneRoot)))
      (Audio|Components|Audio|Play _ms_fireballexplosion 0.0)
      (Class|AudioComponent|SetWaveParameter _ms_fireballexplosion "None" "/Game/SFX/Magic/FireBallExplosion.FireBallExplosion"))
    (:then_1
      ;[1 1 1] Delay slightly before damage
      (Utilities|FlowControl|Delay 0.05)
      ;[1 1 1] Damage
      (bind _outactors (Collision|SphereOverlapActors (Transformation|GetWorldLocation (Variables|Default|GetDefaultSceneRoot)) Radius (Utilities|Array|MakeArray "ObjectTypeQuery1" "ObjectTypeQuery2" "ObjectTypeQuery3" "ObjectTypeQuery4") 0))
      (for _array_element _outactors
        (Utilities|FlowControl|Sequence
          (:then_0
            (Utilities|IsValid (Actor|GetComponentbyClass _array_element "/Game/Player/Blueprints/BPC_Health.BPC_Health_C")
              (:Is%20Valid
                (Class|BPIHealth|TakeDamage(Message) (Actor|GetComponentbyClass _array_element "/Game/Player/Blueprints/BPC_Health.BPC_Health_C") (Math|Float|Truncate Damage) "NewEnumerator2" self))))
          (:then_1
            (bind _asprimitive_component (Utilities|Casting|CastToPrimitiveComponent (Variables|/Script/Engine.Actor|GetRootComponent _array_element)))
            (if (Physics|IsSimulatingPhysics _asprimitive_component "None")
              (Physics|AddForce _asprimitive_component (* (Math|Vector|Normalize (- (Transformation|GetWorldLocation _asprimitive_component) (Transformation|GetWorldLocation (Variables|Default|GetDefaultSceneRoot)))) (/ Radius (Math|Vector|VectorLength (- (Transformation|GetWorldLocation _asprimitive_component) (Transformation|GetWorldLocation (Variables|Default|GetDefaultSceneRoot))))) (Math|Conversions|ToVector(Float) 1e+07)) "None" false)))
          (:then_2
            (Development|PrintString (Utilities|GetDisplayName _array_element))))))
    (:then_2
      (Utilities|FlowControl|Delay 5.0)
      (Actor|DestroyActor))))

(fn ConstructionScript)