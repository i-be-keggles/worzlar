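; BP_Dummy is a physics prop that reacts to taking damage.
; It listens to its health component and pushes the mesh away from the damage source, scaled by damage amount and the unnormalized offset between them.
; Each hit also plays a sound at the mesh through a MetaSound given the hit wave.
; When health is depleted, the physics constraint breaks and the mesh's angular damping drops to zero.
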(event Custom|OnDamaged
  (params (Amount :type Integer) (Type :type E_ElementType%20Enum :default "NewEnumerator0") (Source :type Actor%20Object%20Reference))
  (bind _staticmesh (Variables|Default|GetStaticMesh))
  (Utilities|FlowControl|Sequence
    (:then_0
      (if (<= (Variables|/Game/Util/FunctionalComponents/BPC_Health.BPC_Health_C|GetHealth (Variables|Default|GetBPC_Health)) 0)
        (Class|PhysicsConstraintComponent|BreakConstraint (Variables|Default|GetPhysicsConstraint))
        (Class|PrimitiveComponent|SetAngularDamping (Variables|Default|GetStaticMesh) 0.0)))
    (:then_1
      (Physics|AddForce _staticmesh (* (Math|Conversions|ToVector(Float) 1e+02) Amount (- (Transformation|GetWorldLocation _staticmesh) (Transformation|GetWorldLocation (Variables|/Script/Engine.Actor|GetRootComponent Source)))) "None" true))
    (:then_2
      (bind _returnvalue (Audio|SpawnSoundatLocation "/Game/SFX/Magic/MS_BasicSound.MS_BasicSound" (Transformation|GetWorldLocation (Variables|Default|GetStaticMesh)) "0, 0, 0" 4.0 1.0 0.0 "/Game/SFX/Attenuation/AS_AttenuationMedium.AS_AttenuationMedium" 0))
      (Class|AudioComponent|SetWaveParameter _returnvalue "Sound" "/Game/SFX/Impacts/DummyHit.DummyHit"))))

(event EventBeginPlay
  (EventDispatchers|BindEventtoOnTookDamagePassthrough (Variables|Default|GetBPC_Health) (delegate Custom|OnDamaged)))

(event Collision|EventActorBeginOverlap
  (params (OtherActor :type Actor%20Object%20Reference)))

(event EventTick
  (params (DeltaSeconds :type Float%20%28single-precision%29)))

(fn ConstructionScript)