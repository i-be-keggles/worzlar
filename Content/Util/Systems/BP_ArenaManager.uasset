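; Arena level manager that detects when all enemies are cleared, then runs glyph rewards and the transition to the next level.
; It binds to every EnemySpawner, tracking spawned enemies and their deaths until none remain and spawners are depleted.
; Reward screens chain through selection callbacks, extra rewards before random rounds, then an optional gate triggers saving glyphs and opening NextLevel.
; A debug input destroys enemies and spawners to skip the arena.
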(event Custom|OnEnemySpawned
  (params (Enemy :type BP%20Enemy%20Object%20Reference))
  (Utilities|IsValid Enemy
    (:Is%20Valid
      (EventDispatchers|BindEventtoOnDiedwithReference (Variables|/Game/Enemies/Blueprints/BP_Enemy.BP_Enemy_C|GetBPC_Health Enemy) (delegate Custom|OnEnemyDied))
      (Utilities|Array|Add (Variables|Default|GetEnemies) Enemy))
    (:Is%20Not%20Valid
      (Development|PrintString "Error: enemy not spawned!"))))

(event Custom|OnSpawnerDepleted
  (params (Spawner :type Enemy%20Spawner%20Object%20Reference)))

(event Custom|OnEnemyDied
  (params (HealthComponent :type BPC%20Health%20Object%20Reference))
  (bind _asbp_enemy (Utilities|Casting|CastToBP_Enemy (Components|GetOwner HealthComponent)))
  (Utilities|Array|RemoveItem (Variables|Default|GetEnemies) _asbp_enemy)
  (bind _result (CallFunction|CheckClearedEnemiesandSpawners))
  (if _result
    (CallFunction|CompleteLevel)))

(event Custom|DoExtraRewards
  (bind _hud (Variables|Default|GetHUD))
  (bind _hud_2 (Variables|Default|GetHUD))
  (bind _extrarewards (Variables|Default|GetExtraRewards))
  (bind _wbp_glyphrewardselect (Variables|/Game/UI/Widgets/WBP_HUD.WBP_HUD_C|GetWBP_GlyphRewardSelect _hud_2))
  (if (Utilities|Array|IsEmpty _extrarewards)
    (EventDispatchers|UnbindEventfromOnChoseReward _wbp_glyphrewardselect (delegate Custom|DoExtraRewards))
    (bind _glyphs (Default|ChooseRandomGlyphs _hud 3))
    (Default|ShowReward _hud _glyphs)
    (EventDispatchers|BindEventtoOnChoseReward (Variables|/Game/UI/Widgets/WBP_HUD.WBP_HUD_C|GetWBP_GlyphRewardSelect (stale Custom|CompleteLevel _output_get)) (delegate Custom|SecondaryRewardRounds))
    (else
      (Default|ShowReward _hud_2 (Utilities|Array|MakeArray 0 (Utilities|Array|Get(acopy) _extrarewards) 0))
      (Utilities|Array|RemoveIndex (Variables|Default|GetExtraRewards))
      (EventDispatchers|BindEventtoOnChoseReward _wbp_glyphrewardselect (delegate Custom|DoExtraRewards)))))

(event Custom|CompleteLevel
  (Utilities|FlowControl|Delay 3.0)
  (bind _asbp_first_person_game_mode (Utilities|Casting|CastToBP_FirstPersonGameMode (Game|GetGameMode)))
  (bind _output_get (Variables|Default|SetHUD (Variables|/Game/Player/Blueprints/BP_FirstPersonGameMode.BP_FirstPersonGameMode_C|GetHUD _asbp_first_person_game_mode)))
  (CallFunction|DoExtraRewards))

(event Custom|ProgressToNextLevel
  (bind _returnvalue (Game|GetPlayerController 0))
  (bind _gate (Variables|Default|GetGate))
  (Input|SetInputModeGameandUI _returnvalue 0 "DoNotLock" true false)
  (if (Utilities|IsValidSoftObjectReference (Variables|Default|GetNextLevel))
    (Input|SetInputModeGameOnly _returnvalue false)
    (Utilities|IsValid _gate
      (:Is%20Valid
        (Default|Activate _gate)
        (EventDispatchers|BindEventtoGateUsed _gate (delegate Custom|OnGateUsed)))
      (:Is%20Not%20Valid
        (CallFunction|OnGateUsed)))))

(event Custom|SecondaryRewardRounds
  (bind _hud (Variables|Default|GetHUD))
  (bind _result (Math|Integer|DecrementInt (Variables|Default|GetNumRewardRounds))
    (:%20%20
      (if (> _result 0)
        (bind _glyphs (Default|ChooseRandomGlyphs _hud 3))
        (Default|ShowReward _hud _glyphs)
        (EventDispatchers|BindEventtoOnChoseReward (Variables|/Game/UI/Widgets/WBP_HUD.WBP_HUD_C|GetWBP_GlyphRewardSelect (stale Custom|CompleteLevel _output_get)) (delegate Custom|SecondaryRewardRounds))
        (else
          (CallFunction|ProgresstoNextLevel))))))

(event Custom|OnGateUsed
  (bind _asgi_game_settings (Utilities|Casting|CastToGI_GameSettings (Game|GetGameInstance)))
  (Default|SaveGlyphsfromHUD _asgi_game_settings (Variables|Default|GetHUD))
  (Game|OpenLevel(byObjectReference) (Variables|Default|GetNextLevel)))

(event Input|EnhancedActionEvents|EnhancedInputActionIA_DebugSkipLevel
  (params (ActionValue :type Boolean) (ElapsedSeconds :type Float%20%28double-precision%29) (TriggeredSeconds :type Float%20%28double-precision%29) (InputAction :type Input%20Action%20Object%20Reference :default "/Game/Player/Input/Actions/IA_DebugSkipLevel.IA_DebugSkipLevel"))
  ;[1 1 1] Debug skip level
  (Utilities|FlowControl|DoOnce false
    (:Completed
      (Utilities|FlowControl|Sequence
        (:then_0
          (bind _outactors (Actor|GetAllActorsOfClass "/Game/Enemies/Blueprints/BP_Enemy.BP_Enemy_C"))
          (for _array_element _outactors
            (Actor|DestroyActor _array_element)))
        (:then_1
          (bind _outactors_2 (Actor|GetAllActorsOfClass "/Game/Enemies/Blueprints/EnemySpawner.EnemySpawner_C"))
          (for _array_element_2 _outactors_2
            (Actor|DestroyActor _array_element_2)))
        (:then_2
          (CallFunction|CompleteLevel))))))

(event EventBeginPlay
  (Utilities|FlowControl|Sequence
    (:then_0
      (Input|EnableInput (Game|GetPlayerController 0)))
    (:then_1
      (bind _outactors (Actor|GetAllActorsOfClass "/Game/Enemies/Blueprints/EnemySpawner.EnemySpawner_C"))
      (bind _output_get (Variables|Default|SetEnemySpawners _outactors))
      (for _array_element _output_get
        (EventDispatchers|BindEventtoEnemySpawned _array_element (delegate Custom|OnEnemySpawned))
        (EventDispatchers|BindEventtoSpawnerDepleted _array_element (delegate Custom|OnSpawnerDepleted))))))

(fn ConstructionScript)

(fn CheckClearedEnemiesandSpawners
  (for _array_element (Variables|Default|GetEnemySpawners)
    (if (> (Variables|/Game/Enemies/Blueprints/EnemySpawner.EnemySpawner_C|GetTotalSpawns _array_element) 0)
      (return false)))
  (return (== (Utilities|Array|Length (Variables|Default|GetEnemies)) 0)))