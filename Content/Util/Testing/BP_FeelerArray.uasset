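; BP_FeelerArray is a testing utility actor that lays out a radial array of BP_FeelerNode child actors.
; Its construction script builds concentric rings in the local XZ plane, with Rows setting the ring count and Spacing the radial gap.
; Each ring gains two more nodes than the previous one, spaced evenly by rotating a forward vector around the pitch axis and scaling it by the ring radius.
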(fn ConstructionScript
  (for _index (range 1 (Variables|Default|GetRows))
    (for _index_2 (range 1 (+ (Variables|Default|GetNodes) (* 2 _index)))
      (bind _returnvalue (AddComponent|AddChildActorComponent false (Math|Transform|MakeTransform (* (Class|KismetMathLibrary|QuatVectorForward (Class|KismetMathLibrary|QuatMakefromEuler (Math|Vector|MakeVector 0.0 (* _index_2 (/ 3.6e+02 (Math|Conversions|ToFloat(Integer) (+ (Variables|Default|GetNodes) (* 2 _index))))) 0.0))) _index (Variables|Default|GetSpacing)) "0, 0, 0" "1.000000,1.000000,1.000000")))
      (ChildActorComponent|SetChildActorClass _returnvalue "/Game/Util/Testing/BP_FeelerNode.BP_FeelerNode_C"))))