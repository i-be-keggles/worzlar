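; BP_FeelerNode is a testing actor whose sphere material shows the current health of its health component.
; From BeginPlay it loops HealTick, healing one point every tenth of a second.
; Each tick, and each OnTookDamage event from the component, writes the health fraction to the HealthPercent material parameter on the sphere.
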(event OnTookDamage(BPC_Health)
  (bind _bpc_health (Variables|Default|GetBPC_Health))
  (Rendering|Material|SetScalarParameterValueonMaterials (Variables|Default|GetSphere) "HealthPercent" (/ (Math|Conversions|ToFloat(Integer) (Variables|/Game/Util/FunctionalComponents/BPC_Health.BPC_Health_C|GetHealth _bpc_health)) (Math|Conversions|ToFloat(Integer) (Variables|/Game/Util/FunctionalComponents/BPC_Health.BPC_Health_C|GetMaxHealth _bpc_health)))))

(event Custom|HealTick
  (bind _bpc_health (Variables|Default|GetBPC_Health))
  (Default|Heal (Variables|Default|GetBPC_Health) 1)
  (Utilities|FlowControl|Sequence
    (:then_0
      (Utilities|FlowControl|Delay 0.1)
      (CallFunction|HealTick))
    (:then_1
      (Rendering|Material|SetScalarParameterValueonMaterials (Variables|Default|GetSphere) "HealthPercent" (/ (Math|Conversions|ToFloat(Integer) (Variables|/Game/Util/FunctionalComponents/BPC_Health.BPC_Health_C|GetHealth _bpc_health)) (Math|Conversions|ToFloat(Integer) (Variables|/Game/Util/FunctionalComponents/BPC_Health.BPC_Health_C|GetMaxHealth _bpc_health)))))))

(event EventBeginPlay
  (CallFunction|HealTick))

(fn ConstructionScript)