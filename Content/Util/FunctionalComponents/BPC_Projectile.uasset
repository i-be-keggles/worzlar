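; Projectile component for BP_Glyph actors that drives the glyph's physical root and reports what it hits.
; On BeginPlay it fetches that root from the glyph, optionally disables its collision and sets Active after a short delay.
; Each tick it optionally accelerates the root forward by glyph speed, then sphere-traces along its velocity using glyph size.
; A hit calls OnProjectileHit; with StopOnCollision it also stops physics and destroys itself.
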(event EventBeginPlay
  (bind _asbp_glyph (Utilities|Casting|CastToBP_Glyph (Components|GetOwner)))
  (bind _output_get (Variables|Default|SetGlyph _asbp_glyph))
  (bind _physical_components (Class|BPIGlyph|GetPhysicalRepresentation(Message) _output_get))
  (if (> (Utilities|Array|Length _physical_components) 0)
    (bind _output_get_2 (Variables|Default|SetRoot (Utilities|Array|Get(acopy) _physical_components)))
    (Utilities|FlowControl|Sequence
      (:then_0
        (if (Variables|Default|GetRemoveCollider)
          (Collision|SetCollisionResponsetoAllChannels _output_get_2 "ECR_Ignore")))
      (:then_1
        (Utilities|FlowControl|Delay 0.2)
        (Variables|Default|SetActive true)))))

(event EventTick
  (params (DeltaSeconds :type Float%20%28single-precision%29))
  (bind _glyph (Variables|Default|GetGlyph))
  (bind _root (Variables|Default|GetRoot))
  (bind _root_2 (Variables|Default|GetRoot))
  (bind _returnvalue (Transformation|GetWorldLocation _root_2))
  (bind _speed (Variables|/Game/Magic/Glyphs/Blueprints/BP_Glyph.BP_Glyph_C|GetSpeed _glyph))
  (Utilities|FlowControl|Sequence
    (:then_0
      (if (Variables|Default|GetAccelerative)
        (Utilities|IsValid _root
          (:Is%20Valid
            (Physics|AddForce _root (* DeltaSeconds (Math|Vector|GetForwardVector _root) (Math|Float|SelectFloat 1.0 _speed (<= _speed 0.0)) (Math|Conversions|ToVector(Float) 1e+02) (Variables|Default|GetSpeedMultiplier)) "None" true)))))
    (:then_1
      (bind (_outhit _returnvalue_2) (Collision|SphereTraceByChannel _returnvalue (+ _returnvalue (* (Transformation|GetComponentVelocity _root_2) DeltaSeconds)) (Variables|/Game/Magic/Glyphs/Blueprints/BP_Glyph.BP_Glyph_C|GetSize (Variables|Default|GetGlyph)) "TraceTypeQuery1" false 0 "None"))
      (if _returnvalue_2
        (Utilities|FlowControl|Sequence
          (:then_0
            (Default|CallOnProjectileHit (.hitactor _outhit)))
          (:then_1
            (if (Variables|Default|GetStopOnCollision)
              (Physics|SetSimulatePhysics (Variables|Default|GetRoot) false)
              (Components|DestroyComponent))))))))