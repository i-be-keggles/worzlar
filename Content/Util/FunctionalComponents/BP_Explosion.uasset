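; BP_Explosion is a reusable one-shot explosion actor that deals area damage and knockback, then destroys itself after a few seconds.
; Its Explode event spawns the passed Niagara effect scaled by radius, plays the sound through a MetaSound, then sphere-overlaps after a short delay.
; Each hit actor is processed once, taking flat damage via BPC_Health.
; Physics bodies and character movement receive distance-attenuated outward force; the Knockback input is unused.
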(event Custom|Explode
  (params (Damage :type Float%20%28double-precision%29) (Radius :type Float%20%28double-precision%29) (Knockback :type Float%20%28double-precision%29) (Particles :type Niagara%20System%20Object%20Reference) (Sound :type Sound%20Wave%20Object%20Reference))
  (bind _ms_fireballexplosion (Variables|Default|GetMS_FireballExplosion))
  (bind _hitactors (Variables|Default|GetHitActors))
  (Utilities|FlowControl|Sequence
    (:then_0
      (bind _returnvalue (Niagara|SpawnSystematLocation Particles (Transformation|GetWorldLocation (Variables|Default|GetDefaultSceneRoot))))
      (Effects|Components|ParticleSystem|SetFloatParameter _returnvalue "SizeMultiplier" (/ Radius 4e+02))
      (Class|AudioComponent|SetWaveParameter _ms_fireballexplosion "Sound" Sound)
      (Audio|Parameter|SetFloatParameter _ms_fireballexplosion "PitchVariationMultiplier" 0.5 :!class /Script/AudioExtensions.AudioParameterControllerInterface)
      (Audio|Components|Audio|Play _ms_fireballexplosion 0.0))
    (:then_1
      ;[1 1 1] Delay slightly before damage
      (Utilities|FlowControl|Delay 0.05)
      ;[1 1 1] Damage
      (bind _outcomponents (Collision|SphereOverlapComponents (Transformation|GetWorldLocation (Variables|Default|GetDefaultSceneRoot)) Radius (Utilities|Array|MakeArray "ObjectTypeQuery1" "ObjectTypeQuery2" "ObjectTypeQuery3" "ObjectTypeQuery4")))
      (for _array_element _outcomponents
        (if (not (Utilities|Array|ContainsItem _hitactors (Components|GetOwner _array_element)))
          (Utilities|Array|Add _hitactors (Components|GetOwner _array_element))
          (Utilities|FlowControl|Sequence
            (:then_0
              (Utilities|IsValid (Actor|GetComponentbyClass (Components|GetOwner _array_element) "/Game/Util/FunctionalComponents/BPC_Health.BPC_Health_C")
                (:Is%20Valid
                  (Class|BPIHealth|TakeDamage(Message) (Actor|GetComponentbyClass (Components|GetOwner _array_element) "/Game/Util/FunctionalComponents/BPC_Health.BPC_Health_C") (Math|Float|Truncate Damage) "NewEnumerator2" self))))
            (:then_2
              (if (Physics|IsSimulatingPhysics _array_element "None")
                (Physics|AddForce _array_element (* (Math|Vector|Normalize (- (Transformation|GetWorldLocation _array_element) (Transformation|GetWorldLocation (Variables|Default|GetDefaultSceneRoot)))) (Math|Float|MapRangeClamped (Math|Vector|VectorLength (- (Transformation|GetWorldLocation _array_element) (Transformation|GetWorldLocation (Variables|Default|GetDefaultSceneRoot)))) (* Radius 0.2) Radius 1.0 0.0) (Math|Conversions|ToVector(Float) 1e+07)) "None" false)))
            (:then_3
              (Utilities|IsValid (Actor|GetComponentbyClass (Components|GetOwner _array_element) "/Script/Engine.CharacterMovementComponent")
                (:Is%20Valid
                  (Physics|AddForce (Actor|GetComponentbyClass (Components|GetOwner _array_element) "/Script/Engine.CharacterMovementComponent") (* (Math|Vector|Normalize (- (Transformation|GetWorldLocation _array_element) (Transformation|GetWorldLocation (Variables|Default|GetDefaultSceneRoot)))) (Math|Float|MapRangeClamped (Math|Vector|VectorLength (- (Transformation|GetWorldLocation _array_element) (Transformation|GetWorldLocation (Variables|Default|GetDefaultSceneRoot)))) (* Radius 0.2) Radius 1.0 0.0) (Math|Conversions|ToVector(Float) 1e+07))))))))))
    (:then_2
      (Utilities|FlowControl|Delay 5.0)
      (Actor|DestroyActor))))

(fn ConstructionScript)