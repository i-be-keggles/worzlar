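; A reusable health component that tracks damage, healing and death for its owning actor.
; Damage clamps health at zero, triggers death when it runs out and broadcasts took-damage and died dispatchers, including variants that pass damage details or a self reference.
; A looping one-second timer checks the owner's height and applies a VoidTouch status effect once it falls below a fixed world Z threshold.
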(event Custom|VoidTick
  (bind _returnvalue (Components|GetOwner))
  (if (<= (.z (Transformation|GetWorldLocation (Variables|/Script/Engine.Actor|GetRootComponent _returnvalue))) (Math|Float|MakeLiteralFloat -5e+03))
    (CallFunction|ApplyStatusEffect "/Game/Util/StatusEffects/BPC_StatusEffect_VoidTouch.BPC_StatusEffect_VoidTouch_C" _returnvalue 69.0)))

(event EventBeginPlay
  (Variables|Default|SetHealth (Variables|Default|GetMaxHealth))
  (Utilities|Time|SetTimerbyEvent (delegate Custom|VoidTick) 1.0 true))

(event EventTakeDamage
  (params (Amount :type Integer) (Type :type E_ElementType%20Enum :default "NewEnumerator0") (Source :type Actor%20Object%20Reference))
  (if (> (Variables|Default|GetHealth) 0)
    (bind _output_get (Variables|Default|SetHealth (Math|Integer|Max(Integer) (- (Variables|Default|GetHealth) Amount))))
    (Utilities|FlowControl|Sequence
      (:then_0
        (if (<= _output_get 0)
          (CallFunction|Die)))
      (:then_1
        (Default|CallOnTookDamage)
        (Default|CallOnTookDamagePassthrough Amount Type Source)))))

(event EventDie
  (Default|CallOnDied)
  (Default|CallOnDiedwithReference self))

(event EventHeal
  (params (Amount :type Integer))
  (Variables|Default|SetHealth (Math|Integer|Min(Integer) (+ (Variables|Default|GetHealth) Amount) (Variables|Default|GetMaxHealth))))