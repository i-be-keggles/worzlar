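; Enemy spawner that periodically spawns a weighted-random actor from its Spawnables at its own transform until its spawn budget runs out.
; From BeginPlay, a self-recalling SpawnTick event waits a random delay within the interval range, then spawns regardless of collision.
; Each successful BP_Enemy cast fires EnemySpawned and decrements TotalSpawns, firing SpawnerDepleted at zero.
; A failed cast halts the loop.
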(event Custom|SpawnTick
  (Utilities|FlowControl|Delay (Math|Random|RandomFloatinRange (Variables|Default|GetIntervalMin) (Variables|Default|GetIntervalMax)))
  (bind _randomchoice (CallFunction|RandomWeightedActorClass (Variables|Default|GetSpawnables)))
  (bind _returnvalue (Game|SpawnActorfromClass _randomchoice (Transformation|GetActorTransform) "AlwaysSpawn" "MultiplyWithRoot" 0 0))
  (bind _asbp_enemy (Utilities|Casting|CastToBP_Enemy _returnvalue))
  (Default|CallEnemySpawned _asbp_enemy)
  (bind _result (Math|Integer|DecrementInt (Variables|Default|GetTotalSpawns))
    (:%20%20
      (if (== _result 0)
        (Default|CallSpawnerDepleted self)
        (else
          (CallFunction|SpawnTick))))))

(event EventBeginPlay
  (CallFunction|SpawnTick))

(fn ConstructionScript)