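; AI controller for a flying enemy that chases the player and dashes at them when close and facing them.
; Chase loops each tick, using a downward trace for hover force, then interpolating yaw, damping sideways drift and accelerating forward with capsule physics forces.
; Dash spawns a Niagara effect, calls the attack and launches the enemy toward the player, then resumes chasing with temporarily reduced turn speed.
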(event Custom|Dash
  (bind _enemy (Variables|Default|GetEnemy))
  (bind _capsulecomponent (Variables|/Script/Engine.Character|GetCapsuleComponent _enemy))
  (bind _returnvalue (Transformation|GetWorldLocation _capsulecomponent))
  (Utilities|FlowControl|Sequence
    (:then_0
      (Niagara|SpawnSystematLocation "/Game/VFX/NiagaraSystems/NS_Dash.NS_Dash" _returnvalue (Math|Conversions|RotationFromXVector (Math|Vector|NegateVector (Math|Vector|GetForwardVector _capsulecomponent)))))
    (:then_1
      (Default|CallOnAttack))
    (:then_2
      (Physics|AddForce _capsulecomponent (* (Math|Conversions|ToVector(Float) 1e+05) (Math|Vector|Normalize (- (Transformation|GetActorLocation (Variables|Default|GetPlayer)) _returnvalue))) "None" true)
      (Utilities|FlowControl|Delay 2.0)
      (Variables|Default|SetTurnSpeed 2.0)
      (CallFunction|Chase)
      (Utilities|FlowControl|Delay 2.0)
      (Variables|Default|SetTurnSpeed 1e+01))))

(event EventBeginPlay
  (|CallParentFunction) ; This node is disabled and will not be called.\nDrag off pins to build functionality.
)

(event EventChase
  (bind _enemy (Variables|Default|GetEnemy))
  (bind _enemy_2 (Variables|Default|GetEnemy))
  (bind _enemy_3 (Variables|Default|GetEnemy))
  (bind _enemy_4 (Variables|Default|GetEnemy))
  (bind _enemy_5 (Variables|Default|GetEnemy))
  (bind _returnvalue (Transformation|GetActorLocation _enemy_5))
  (bind _capsulecomponent (Variables|/Script/Engine.Character|GetCapsuleComponent _enemy))
  (bind _returnvalue_2 (Transformation|GetComponentVelocity _capsulecomponent))
  (Utilities|IsValid (Variables|Default|GetPlayer)
    (:Is%20Valid
      (Utilities|FlowControl|Sequence
        (:then_0
          (bind (_outhit _returnvalue_3) (Collision|LineTraceByChannel _returnvalue (- _returnvalue (Math|Vector|MakeVector 0.0 0.0 (* (Variables|Default|GetHoverHeight) 5.0))) "TraceTypeQuery1" false (Utilities|Array|MakeArray (Variables|Default|GetEnemy)) "None"))
          (if _returnvalue_3
            (Physics|AddForce (Variables|/Script/Engine.Character|GetCapsuleComponent (Variables|Default|GetEnemy)) (Math|Vector|MakeVector 0.0 0.0 (* (- (Variables|Default|GetHoverHeight) (.distance _outhit)) (Utilities|Time|GetWorldDeltaSeconds) 1e+02)) "None" true)))
        (:then_1
          ;[1 1 1] Rotate
          (Transformation|SetActorRotation _enemy_2 (Math|Rotator|MakeRotator 0.0 0.0 (.yaw (Math|Interpolation|RInterpTo (Transformation|GetActorRotation _enemy_2) (Math|Rotator|FindLookatRotation (Transformation|GetActorLocation _enemy_2) (Transformation|GetActorLocation (Variables|Default|GetPlayer))) (Utilities|Time|GetWorldDeltaSeconds) (Variables|Default|GetTurnSpeed)))))
          ;[1 1 1] Stabilise drift
          (Physics|AddForce _capsulecomponent (* (Math|Vector|ProjectVectorontoVector _returnvalue_2 (Math|Vector|GetRightVector _capsulecomponent)) (Utilities|Time|GetWorldDeltaSeconds) (Math|Conversions|ToVector(Float) -2e+02)) "None" true)
          ;[1 1 1] Forward
          (if (< (Math|Vector|VectorLength _returnvalue_2) (Variables|Default|GetSpeed))
            (Physics|AddForce (Variables|/Script/Engine.Character|GetCapsuleComponent _enemy_3) (* (Transformation|GetActorForwardVector _enemy_3) (Utilities|Time|GetWorldDeltaSeconds) 1e+03 (Variables|Default|GetAcceleration)) "None" true)))
        (:then_2
          ;[1 1 1] Fix root location
          (Transformation|SetActorLocation _enemy_4 (Transformation|GetWorldLocation (Variables|/Script/Engine.Character|GetCapsuleComponent _enemy_4)) false true))
        (:then_3
          (bind _result (CallFunction|IsFacingPlayer 2e+01))
          (bind _distance (CallFunction|DistancetoPlayer))
          (if (and (<= _distance 5e+02) _result)
            (CallFunction|Dash)
            (else
              (Utilities|FlowControl|DelayUntilNextTick)
              (CallFunction|Chase))))))))

(fn ConstructionScript
  (|CallParentFunction))