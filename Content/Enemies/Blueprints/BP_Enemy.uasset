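; BP_Enemy is an enemy character that attacks on command from AIC_EnemyController and reacts to damage and death.
; Attack IDs index montages, spawned attack classes and offsets; non-animation-based attacks spawn from the montage's then pin.
; Health component events drive flinch feedback, controller notification, and death with material-matched chunk particles and a chance of a health pickup.
; Sounds feed per-enemy waves into MetaSound parameters.
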(event OnTookDamagePassthrough(BPC_Health)
  (params (Amount :type Integer) (Type :type E_ElementType%20Enum :default "NewEnumerator0") (Source :type Actor%20Object%20Reference))
  (bind _returnvalue (Audio|SpawnSoundatLocation "/Game/SFX/Metasounds/MS_BasicVariation.MS_BasicVariation" (Transformation|GetActorLocation) "0, 0, 0" 1.0 1.0 0.0 "/Game/SFX/Attenuation/AS_AttenuationMedium.AS_AttenuationMedium" 0))
  (Class|AudioComponent|SetWaveParameter _returnvalue "Sound" (Variables|Default|GetFlinchSound))
  (Animation|Montage|PlayMontage (Variables|Character|GetMesh) (Variables|Default|GetFlinchAnimation)
    (:then
      (Default|OnTakeDamage (Variables|Default|GetAIController)))))

(event OnDied(BPC_Health)
  (Utilities|FlowControl|Sequence
    (:then_0
      (if (Math|Random|RandomBoolwithWeight 0.15)
        (Game|SpawnActorfromClass "/Game/Util/FunctionalComponents/BP_HealthPickup.BP_HealthPickup_C" (Math|Transform|MakeTransform (Transformation|GetActorLocation) "0, 0, 0" "1.000000,1.000000,1.000000") "Undefined" "MultiplyWithRoot" 0 0)))
    (:then_1
      (bind _returnvalue (Audio|SpawnSoundatLocation "/Game/SFX/Metasounds/MS_BasicVariation.MS_BasicVariation" (Transformation|GetActorLocation) "0, 0, 0" 1.0 1.0 0.0 "/Game/SFX/Attenuation/AS_AttenuationMedium.AS_AttenuationMedium" 0))
      (Class|AudioComponent|SetWaveParameter _returnvalue "Sound" (Variables|Default|GetDeathSound)))
    (:then_2
      (Variables|/Script/Engine.CharacterMovementComponent|SetMaxWalkSpeed (Variables|Character|GetCharacterMovement) 0.0)
      (bind _returnvalue_2 (Niagara|SpawnSystematLocation "/Game/VFX/NiagaraSystems/NS_EnemyChunks.NS_EnemyChunks" (Transformation|GetActorLocation)))
      (Class|NiagaraComponent|SetVariableMaterial _returnvalue_2 "Material" (Rendering|Material|GetMaterial (Variables|Character|GetMesh) 0))
      (Utilities|FlowControl|Delay 0.2)
      (Actor|DestroyActor))))

(event Custom|OnStartAttack
  (params (AttackID :type Integer))
  (Animation|Montage|PlayMontage (Variables|Character|GetMesh) (Utilities|Array|Get(acopy) (Variables|Default|GetAttackAnimations) AttackID)
    (:then
      (bind _returnvalue (Audio|SpawnSoundatLocation "/Game/SFX/Metasounds/MS_BasicVariation.MS_BasicVariation" (Transformation|GetActorLocation) "0, 0, 0" 1.0 1.0 0.0 "/Game/SFX/Attenuation/AS_AttenuationMedium.AS_AttenuationMedium" 0))
      (Class|AudioComponent|SetWaveParameter _returnvalue "Sound" (Variables|Default|GetAttackSound))
      (if (not (.AnimationBased (Utilities|GetClassDefaults (Utilities|Array|Get(acopy) (Variables|Default|GetAttacks) AttackID))))
        (CallFunction|Attack AttackID)))))

(event EventBeginPlay
  (Class|AudioComponent|SetWaveParameter (Variables|Default|GetFootsteps) "Sound" (Variables|Default|GetFootstepSound)))

(event EventPossessed
  (params (NewController :type Controller%20Object%20Reference))
  (bind _asaic_enemy_controller (Utilities|Casting|CastToAIC_EnemyController NewController))
  (bind _output_get (Variables|Default|SetAIController _asaic_enemy_controller))
  (EventDispatchers|BindEventtoOnAttack _output_get (delegate Custom|OnStartAttack)))

(event EventNotifyFootstep
  (Audio|Components|Audio|Play (Variables|Default|GetFootsteps) 0.0))

(event EventAttack
  (params (AttackID :type Integer))
  (bind _capsulecomponent (Variables|Collision|GetCapsuleComponent))
  (Game|SpawnActorfromClass (Utilities|Array|Get(acopy) (Variables|Default|GetAttacks) AttackID) (Math|Transform|MakeTransform (Math|Transform|TransformLocation (Transformation|GetWorldTransform _capsulecomponent) (Utilities|Array|Get(acopy) (Variables|Default|GetAttackOffsets) AttackID)) (Transformation|GetWorldRotation _capsulecomponent) "1.000000,1.000000,1.000000") "Undefined" "MultiplyWithRoot" 0 self 0))

(fn ConstructionScript)