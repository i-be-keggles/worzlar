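; AI controller for BP_Enemy that chases and attacks the player through a delay-driven event loop.
; Chase turns the enemy when the player is close but outside its facing angle, otherwise runs AIMoveTo and retries on failure.
; Finishing a move fires the OnAttack dispatcher unless stunned, then resumes the chase after a cooldown.
; Taking damage briefly stuns the enemy, halting movement before Chase restarts.
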(event Custom|Attack
  (Default|CallOnAttack)
  (Utilities|FlowControl|Delay 2.0)
  (CallFunction|Chase))

(event Custom|Chase
  (if (Utilities|IsValid (Variables|Default|GetPlayer))
    (bind (_result _rotationtoplayer) (CallFunction|IsFacingPlayer 3e+01))
    (bind _distance (CallFunction|DistancetoPlayer))
    (if (and (< _distance 5e+02) (not _result))
      (Pawn|SetControlRotation _rotationtoplayer)
      (Utilities|FlowControl|Delay 0.2)
      (CallFunction|Chase)
      (else
        (AI|AIMoveTo self "0, 0, 0" (Variables|Default|GetPlayer) -1.0 "Default" "Default" true true
          (:OnRequestFailed
            (Development|PrintString "Failed")
            (Utilities|FlowControl|Delay 3.0)
            (CallFunction|Chase))
          (:OnMoveFinished
            (if (not (Variables|Default|GetStunned))
              (Development|PrintString "Finished movement.")
              (CallFunction|Attack))))))
    (else
      (Utilities|FlowControl|Delay 0.2)
      (CallFunction|Chase))))

(event Custom|OnTakeDamage
  (CallFunction|Stun 0.6))

(event Custom|Stun
  (params (Duration :type Float%20%28double-precision%29))
  (bind _enemy (Variables|Default|GetEnemy))
  (Variables|Default|SetStunned true)
  (AI|AIMoveTo _enemy "0, 0, 0" _enemy 5.0 false
    (:then
      (AI|Navigation|StopMovement)
      (Utilities|FlowControl|Delay Duration)
      (Variables|Default|SetStunned false)
      (CallFunction|Chase))))

(event EventPossess
  (params (PossessedPawn :type Pawn%20Object%20Reference))
  (Utilities|FlowControl|Sequence
    (:then_0
      (bind _asbp_player (Utilities|Casting|CastToBP_Player (Game|Player|GetPlayerPawn 0)))
      (Variables|Default|SetPlayer _asbp_player))
    (:then_1
      (bind _asbp_enemy (Utilities|Casting|CastToBP_Enemy (Pawn|GetControlledPawn)))
      (Variables|Default|SetEnemy _asbp_enemy))
    (:then_2
      (Utilities|IsValid (Variables|Default|GetPlayer)
        (:Is%20Valid
          (Utilities|IsValid (Variables|Default|GetEnemy)
            (:Is%20Valid
              (CallFunction|Chase))))))))

(event EventBeginPlay
  (Utilities|FlowControl|Sequence
    (:then_0
      (bind _asbp_player (Utilities|Casting|CastToBP_Player (Game|Player|GetPlayerPawn 0)))
      (Variables|Default|SetPlayer _asbp_player))
    (:then_1
      (bind _asbp_enemy (Utilities|Casting|CastToBP_Enemy (Pawn|GetControlledPawn)))
      (Variables|Default|SetEnemy _asbp_enemy))
    (:then_2
      (Utilities|IsValid (Variables|Default|GetPlayer)
        (:Is%20Valid
          (Utilities|IsValid (Variables|Default|GetEnemy)
            (:Is%20Valid
              (CallFunction|Chase))))))))

(fn ConstructionScript)

(fn IsFacingPlayer
  (params (Angle :type Float%20%28double-precision%29))
  (bind _enemy (Variables|Default|GetEnemy))
  (bind _player (Variables|Default|GetPlayer))
  (bind _returnvalue (Transformation|GetActorLocation _enemy))
  (bind _returnvalue_2 (Transformation|GetActorLocation _player))
  (bind _returnvalue_3 (Math|Rotator|FindLookatRotation _returnvalue _returnvalue_2))
  (return (< (Math|Float|Absolute(Float) (- (.yaw (Transformation|GetActorRotation _enemy)) (.Yaw (Math|Rotator|BreakRotator _returnvalue_3)))) Angle) _returnvalue_3))

(fn DistancetoPlayer
  (return (Math|Vector|Distance(Vector) (Transformation|GetActorLocation (Variables|Default|GetEnemy)) (Transformation|GetActorLocation (Variables|Default|GetPlayer)))))