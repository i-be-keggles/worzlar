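; AI controller for the Angel enemy, with a Chase event that picks between melee and ranged attacks on the player.
; Inside melee radius it turns if needed when in attack range, or moves to the player, then attacks unless stunned.
; Farther away it line-traces from the attack offset height, stopping to face and fire a projectile on a hit, otherwise moving closer.
; Turning, failed moves and repositioning re-enter Chase after delays.
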(event EventBeginPlay
  (|CallParentFunction) ; This node is disabled and will not be called.\nDrag off pins to build functionality.
)

(event EventChase
  (bind _player (Variables|Default|GetPlayer))
  (bind _enemy (Variables|Default|GetEnemy))
  (if (Utilities|IsValid (Variables|Default|GetPlayer))
    (bind (_result _rotationtoplayer) (CallFunction|IsFacingPlayer 3e+01))
    (bind _distance (CallFunction|DistancetoPlayer))
    (if (<= _distance (Variables|Default|GetMeleeRadius))
      (if (and (< _distance (Variables|Default|GetAttackRange)) (not _result))
        (Pawn|SetControlRotation _rotationtoplayer :!label _label)
        (Utilities|FlowControl|Delay 0.2)
        (CallFunction|Chase)
        (else
          (AI|AIMoveTo self "0, 0, 0" (Variables|Default|GetPlayer) -1.0 "Default" "Default" true true
            (:OnRequestFailed
              (Development|PrintString "Failed")
              (Utilities|FlowControl|Delay 3.0)
              (CallFunction|Chase))
            (:OnMoveFinished
              (if (not (Variables|Default|GetStunned))
                (CallFunction|Attack))))))
      (else
        (Utilities|FlowControl|Sequence
          (:then_0
            (bind _outhit (Collision|LineTraceByChannel (+ (Transformation|GetActorLocation (Variables|Default|GetEnemy)) (* (Utilities|Array|Get(acopy) (Variables|/Game/Enemies/Blueprints/BP_Enemy.BP_Enemy_C|GetAttackOffsets _enemy) 1) "0.000000,0.000000,1.000000")) (Transformation|GetActorLocation _player) "TraceTypeQuery3" false (Utilities|Array|MakeArray _enemy) "None" true "(R=1.000000,G=0.000000,B=0.000000,A=1.000000)" "(R=0.000000,G=1.000000,B=0.000000,A=1.000000)" 1.0))
            (if (== (.HitActor (Collision|BreakHitResult _outhit)) _player)
              (AI|Navigation|StopMovement)
              (bind _result_2 (CallFunction|IsFacingPlayer 1e+01))
              (if _result_2
                (CallFunction|Attack 1)
                (Development|PrintString "Projectiling")
                (else
                  (goto _label)))
              (else
                (AI|AIMoveTo 0 "0, 0, 0" (Variables|Default|GetPlayer) -1.0 "Default" "Default" true false
                  (:then
                    (Utilities|FlowControl|Delay 1.0)
                    (CallFunction|Chase)))))))))
    (else
      (Utilities|FlowControl|Delay 0.2)
      (CallFunction|Chase))))

(fn ConstructionScript
  (|CallParentFunction))