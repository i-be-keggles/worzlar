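; Fish enemy Blueprint that deals contact damage during a short dash attack.
; Starting an attack calls the parent logic, then holds a Dashing flag on for a fixed delay.
; While dashing, a capsule hit on an actor with a BPC_Health component applies damage and clears the flag, ending the damage window early.
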(event OnComponentHit(Capsule)
  (params (HitComponent :type Primitive%20Component%20Object%20Reference) (OtherActor :type Actor%20Object%20Reference) (OtherComp :type Primitive%20Component%20Object%20Reference) (NormalImpulse :type Vector :default "0, 0, 0") (Hit :type Hit%20Result%20Structure%20%28by%20ref%29))
  (bind _returnvalue (Actor|GetComponentbyClass OtherActor "/Game/Util/FunctionalComponents/BPC_Health.BPC_Health_C"))
  (if (Variables|Default|GetDashing)
    (Utilities|IsValid _returnvalue
      (:Is%20Valid
        (Default|TakeDamage _returnvalue 20 "NewEnumerator0" self)
        (Variables|Default|SetDashing false)))))

(event EventOnStartAttack
  (params (AttackID :type Integer))
  (|CallParentFunction AttackID)
  (Variables|Default|SetDashing true)
  (Utilities|FlowControl|Delay 1.0)
  (Variables|Default|SetDashing false))

(fn ConstructionScript
  (|CallParentFunction))