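; AI controller for a teleporting enemy that turns toward the player, attacks and jumps to random spots around them.
; Chase re-runs each tick, smoothing yaw and calling Teleport after a delay when the player is close.
; Attacks require facing and a clear sphere trace, with tracking locked partway through and a cooldown afterward.
; Teleport picks a random horizontal offset plus height, and a looping BeginPlay debug timer also triggers it.
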(event Custom|TP_Debug
  (CallFunction|Teleport))

(event EventBeginPlay
  (|CallParentFunction)
  (Utilities|Time|SetTimerbyEvent (delegate Custom|TP_Debug) 2e+01 true))

(event EventChase
  (bind _enemy (Variables|Default|GetEnemy))
  (bind _attacktrackingstop (Variables|Default|GetAttackTrackingStop))
  (bind _enemy_2 (Variables|Default|GetEnemy))
  (bind _enemy_3 (Variables|Default|GetEnemy))
  (bind _player (Variables|Default|GetPlayer))
  (bind _attacktrackingdopercent (Variables|Default|GetAttackTrackingDoPercent))
  (bind _returnvalue (* _attacktrackingstop _attacktrackingdopercent))
  (Utilities|IsValid (Variables|Default|GetPlayer)
    (:Is%20Valid
      (Utilities|FlowControl|Sequence
        (:then_1
          ;[1 1 1] Rotate
          (if (not (Variables|Default|GetAttacking))
            (Transformation|SetActorRotation _enemy (Math|Rotator|MakeRotator 0.0 0.0 (.yaw (Math|Interpolation|RInterpTo (Transformation|GetActorRotation _enemy) (Math|Rotator|FindLookatRotation (Transformation|GetActorLocation _enemy) (Transformation|GetActorLocation (Variables|Default|GetPlayer))) (Utilities|Time|GetWorldDeltaSeconds) (Variables|Default|GetTurnSpeed)))))))
        (:then_2
          ;[1 1 1] Fix root location
          (Transformation|SetActorLocation _enemy_2 (Transformation|GetWorldLocation (Variables|/Script/Engine.Character|GetCapsuleComponent _enemy_2)) false true))
        (:then_3
          (bind _distance (CallFunction|DistancetoPlayer))
          (if (<= _distance 1e+03)
            (Utilities|FlowControl|Delay 2.0)
            (CallFunction|Teleport)))
        (:then_4
          (if (Variables|Default|GetCanAttack)
            (bind _result (CallFunction|IsFacingPlayer 5.0))
            (if _result
              (bind _outhit (Collision|SphereTraceByChannel (Transformation|GetActorLocation _enemy_3) (Transformation|GetActorLocation _player) 2e+01 "TraceTypeQuery3" false (Utilities|Array|MakeArray _enemy_3) "None"))
              (if (== (.HitActor (Collision|BreakHitResult _outhit)) _player)
                (CallFunction|Attack)
                (Variables|Default|SetCanAttack false)
                (Utilities|FlowControl|Delay _returnvalue)
                (Variables|Default|SetAttacking true)
                (Utilities|FlowControl|Delay (- _attacktrackingstop _returnvalue))
                (Variables|Default|SetAttacking false)
                (Utilities|FlowControl|Delay 4.0)
                (Variables|Default|SetCanAttack true)))))
        (:then_5
          (Utilities|FlowControl|DelayUntilNextTick)
          (CallFunction|Chase))))))

(fn ConstructionScript
  (|CallParentFunction))

(fn Teleport
  (bind _minteleportrange (Variables|Default|GetMinTeleportRange))
  (bind _maxteleportrange (Variables|Default|GetMaxTeleportRange))
  (bind _returnvalue (Math|Random|RandomFloatinRange _minteleportrange _maxteleportrange))
  (Development|PrintString "Teleporting")
  (Transformation|SetActorLocation (Variables|Default|GetEnemy) (+ (+ (Transformation|GetActorLocation (Variables|Default|GetPlayer)) (* (Math|Vector|Normalize (* (Math|Random|RandomUnitVector) "1.000000,1.000000,0.000000")) _returnvalue)) (Math|Vector|MakeVector 0.0 0.0 (Math|Random|RandomFloatinRange 0.0 (Math|Float|MapRangeClamped _returnvalue _minteleportrange _maxteleportrange (Math|Float|MapRangeClamped _returnvalue _minteleportrange _maxteleportrange 0.0 6e+02) 1e+03)))) false true))