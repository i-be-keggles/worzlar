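; BP_EnemyAttack_Projectile is an enemy attack projectile that can optionally aim at the player when it spawns.
; On BeginPlay it hands its Collision to the projectile component and spawns a BP_Glyph, passing it Speed and Radius as size.
; When the component reports a hit, it spawns a Niagara burst, damages any BPC_Health on the hit result, then destroys the glyph and, a tick later, itself.
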(event OnProjectileHit(BPC_Projectile)
  (params (Hit :type Actor%20Object%20Reference))
  (bind _returnvalue (Actor|GetComponentbyClass Hit "/Game/Util/FunctionalComponents/BPC_Health.BPC_Health_C"))
  (Niagara|SpawnSystematLocation "/Game/VFX/NiagaraSystems/NS_MagicBurstLarge.NS_MagicBurstLarge" (Transformation|GetWorldLocation (Variables|Default|GetCollision)))
  (Utilities|FlowControl|Sequence
    (:then_0
      (Utilities|IsValid _returnvalue
        (:Is%20Valid
          (Class|BPIHealth|TakeDamage(Message) _returnvalue (Variables|Default|GetDamage) (Variables|Default|GetDamageType) self))))
    (:then_1
      (Actor|DestroyActor (Variables|Default|GetDummyGlyph))
      (Utilities|FlowControl|DelayUntilNextTick)
      (Actor|DestroyActor))))

(event EventBeginPlay
  (bind _collision (Variables|Default|GetCollision))
  (bind _bpc_projectile (Variables|Default|GetBPC_Projectile))
  (Utilities|FlowControl|Sequence
    (:then_0
      (if (Variables|Default|GetStartAlignedToPlayer)
        (Transformation|SetWorldTransform _collision (Class|KismetAnimationLibrary|Lookat (Transformation|GetWorldTransform _collision) (Transformation|GetActorLocation (Game|Player|GetPlayerPawn 0)) "1.000000,0.000000,0.000000" false "0, 0, 0" 0.0) false false)))
    (:then_1
      (Variables|/Game/Util/FunctionalComponents/BPC_Projectile.BPC_Projectile_C|SetRoot _bpc_projectile (Variables|Default|GetCollision))
      (bind _returnvalue (Game|SpawnActorfromClass "/Game/Magic/Glyphs/Blueprints/BP_Glyph.BP_Glyph_C" (Transformation|GetActorTransform) "Undefined" "MultiplyWithRoot" 0 0))
      (bind _output_get (Variables|/Game/Util/FunctionalComponents/BPC_Projectile.BPC_Projectile_C|SetGlyph _bpc_projectile _returnvalue))
      (bind _output_get_2 (Variables|Default|SetDummyGlyph _output_get))
      (Variables|/Game/Magic/Glyphs/Blueprints/BP_Glyph.BP_Glyph_C|SetSpeed _output_get_2 (Variables|Default|GetSpeed))
      (Variables|/Game/Magic/Glyphs/Blueprints/BP_Glyph.BP_Glyph_C|SetSize _output_get_2 (Variables|Default|GetRadius)))))

(fn ConstructionScript
  (|CallParentFunction))