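; Homing enemy projectile that chases the player and deals damage on impact.
; It moves by physics: an upward kick on BeginPlay, then an acceleration force every tick from its collision component toward the player pawn, scaled by Speed.
; Hitting anything other than its owning Enemy sends damage to that actor's BPC_Health component, if present, then destroys the projectile.
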(event OnComponentHit(Collision)
  (params (HitComponent :type Primitive%20Component%20Object%20Reference) (OtherActor :type Actor%20Object%20Reference) (OtherComp :type Primitive%20Component%20Object%20Reference) (NormalImpulse :type Vector :default "0, 0, 0") (Hit :type Hit%20Result%20Structure%20%28by%20ref%29))
  (bind _returnvalue (Actor|GetComponentbyClass OtherActor "/Game/Util/FunctionalComponents/BPC_Health.BPC_Health_C"))
  (if (!= OtherActor (Variables|Default|GetEnemy))
    (Utilities|FlowControl|Sequence
      (:then_0
        (Utilities|IsValid _returnvalue
          (:Is%20Valid
            (Class|BPIHealth|TakeDamage(Message) _returnvalue (Variables|Default|GetDamage) (Variables|Default|GetDamageType) self))))
      (:then_1
        (Actor|DestroyActor)))))

(event EventTick
  (params (DeltaSeconds :type Float%20%28single-precision%29))
  (bind _collision (Variables|Default|GetCollision))
  (Physics|AddForce _collision (* (Variables|Default|GetSpeed) (Math|Vector|Normalize (- (Transformation|GetActorLocation (Variables|Default|GetPlayer)) (Transformation|GetWorldLocation _collision)))) "None" true))

(event EventBeginPlay
  (Physics|AddForce (Variables|Default|GetCollision) "0.000000,0.000000,10000.000000" "None" true)
  (Variables|Default|SetPlayer (Game|Player|GetPlayerPawn 0)))

(fn ConstructionScript
  (|CallParentFunction))