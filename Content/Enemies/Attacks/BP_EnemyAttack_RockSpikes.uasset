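; Enemy attack actor that spawns a ring of rock spikes around its location to damage what they hit.
; On BeginPlay it spawns evenly spaced, tilted BP_RockSpike actors at Radius and binds each HitTrigger overlap.
; Overlaps send damage through BPC_Health to any actor that has one, except the owning Enemy.
; After a short delay it retracts all spikes and destroys itself.
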(event Custom|OnSpikeHit
  (params (OverlappedComponent :type Primitive%20Component%20Object%20Reference) (OtherActor :type Actor%20Object%20Reference) (OtherComp :type Primitive%20Component%20Object%20Reference) (OtherBodyIndex :type Integer) (bFromSweep :type Boolean) (SweepResult :type Hit%20Result%20Structure%20%28by%20ref%29))
  (bind _returnvalue (Actor|GetComponentbyClass OtherActor "/Game/Util/FunctionalComponents/BPC_Health.BPC_Health_C"))
  (if (!= OtherActor (Variables|Default|GetEnemy))
    (Utilities|IsValid _returnvalue
      (:Is%20Valid
        (Class|BPIHealth|TakeDamage(Message) _returnvalue (Variables|Default|GetDamage) (Variables|Default|GetDamageType) self)))))

(event EventBeginPlay
  (Utilities|FlowControl|Sequence
    (:then_0
      (for _index (range 1 (Variables|Default|GetNSpikes))
        (bind _returnvalue (Game|SpawnActorfromClass "/Game/Enemies/Attacks/Models/BP_RockSpike.BP_RockSpike_C" (Math|Transform|MakeTransform (+ (Transformation|GetActorLocation) (Math|Vector|RotateVectorAroundAxis (Math|Vector|MakeVector (Variables|Default|GetRadius) 0.0 0.0) (* _index (/ 360 (Variables|Default|GetNSpikes))) "0.000000,0.000000,1.000000")) (Math|Rotator|MakeRotator 0.0 -15.0 (* _index (/ 360 (Variables|Default|GetNSpikes)))) "1.000000,1.000000,1.000000") "Undefined" "MultiplyWithRoot" 0 0))
        (Utilities|Array|Add (Variables|Default|GetSpikes) _returnvalue)
        (Collision|BindEventtoOnComponentBeginOverlap (Variables|/Game/Enemies/Attacks/Models/BP_RockSpike.BP_RockSpike_C|GetHitTrigger _returnvalue) (delegate Custom|OnSpikeHit))))
    (:then_1
      (Utilities|FlowControl|Delay 3.0)
      (for _array_element (Variables|Default|GetSpikes)
        (Default|Retract _array_element true))
      (Actor|DestroyActor))))

(fn ConstructionScript
  (|CallParentFunction))