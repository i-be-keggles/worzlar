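; BP_EnemyAttack_GroundSlam is an enemy ground slam attack that deals one burst of area damage when it begins play.
; A sphere overlap at the Sphere component's location gathers pawns within Radius, ignoring the Enemy reference.
; Each pawn with a BPC_Health component receives a TakeDamageMessage carrying Damage and DamageType, with the attack itself as source.
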(event EventBeginPlay
  (bind _outactors (Collision|SphereOverlapActors (Transformation|GetWorldLocation (Variables|Default|GetSphere)) (Variables|Default|GetRadius) (Utilities|Array|MakeArray "ObjectTypeQuery3") 0 (Utilities|Array|MakeArray (Variables|Default|GetEnemy))))
  (for _array_element _outactors
    (Utilities|IsValid (Actor|GetComponentbyClass _array_element "/Game/Util/FunctionalComponents/BPC_Health.BPC_Health_C")
      (:Is%20Valid
        (Class|BPIHealth|TakeDamage(Message) (Actor|GetComponentbyClass _array_element "/Game/Util/FunctionalComponents/BPC_Health.BPC_Health_C") (Variables|Default|GetDamage) (Variables|Default|GetDamageType) self)))))

(fn ConstructionScript
  (|CallParentFunction))