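; Enemy laser attack actor that, after a windup, fires a beam along its forward axis and damages whatever it hits.
; It attaches to its enemy and aims at the player on spawn and again a second later.
; A sphere trace then sets the Niagara beam length, triggers impact audio and sends briefly delayed damage to BPC_Health.
; It detaches when firing and destroys itself on a fixed timer started at spawn.
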(event Custom|TrackTimer
  (Utilities|FlowControl|Delay 1.0)
  (Transformation|SetActorRotation (Math|Rotator|FindLookatRotation (Transformation|GetActorLocation) (Transformation|GetActorLocation (Game|Player|GetPlayerPawn 0))))
  (Transformation|AttachActorToActor (Variables|Default|GetEnemy) "None" "KeepWorld" "KeepWorld" "KeepWorld" true))

(event EventBeginPlay
  (bind _returnvalue (Transformation|GetActorLocation))
  (bind _returnvalue_2 (Transformation|GetActorForwardVector))
  (CallFunction|TrackTimer)
  (Utilities|FlowControl|Sequence
    (:then_0
      (Transformation|SetActorRotation (Math|Rotator|FindLookatRotation (Transformation|GetActorLocation) (Transformation|GetActorLocation (Game|Player|GetPlayerPawn 0))))
      (Transformation|AttachActorToActor (Variables|Default|GetEnemy) "None" "KeepWorld" "KeepWorld" "KeepWorld" true))
    (:then_1
      (Utilities|FlowControl|Delay (Variables|Default|GetWindup%20Time))
      (bind (_outhit _returnvalue_3) (Collision|SphereTraceByChannel (+ _returnvalue (* (Math|Conversions|ToVector(Float) 3e+02) _returnvalue_2)) (+ _returnvalue (* _returnvalue_2 (Variables|Default|GetRange))) (Variables|Default|GetRadius) "TraceTypeQuery3" false (Utilities|Array|MakeArray (Variables|Default|GetEnemy)) "None" true "(R=1.000000,G=0.000000,B=0.000000,A=1.000000)" "(R=0.000000,G=1.000000,B=0.000000,A=1.000000)" 1.0))
      (Utilities|FlowControl|Sequence
        (:then_0
          (Transformation|DetachFromActor "KeepWorld" "KeepWorld" "KeepWorld"))
        (:then_1
          (bind _returnvalue_4 (Niagara|SpawnSystemAttached "/Game/VFX/NiagaraSystems/NS_Laserbeam.NS_Laserbeam" (Variables|Default|GetDefaultSceneRoot) "None" "0, 0, 0" "0, 0, 0" "SnapToTarget" false))
          (Effects|Components|ParticleSystem|SetFloatParameter _returnvalue_4 "Length" (+ (/ (.distance _outhit) 1e+02) 3.0))
          (Transformation|SetRelativeRotation _returnvalue_4 "-90.000000,0.000000,0.000000" false false)
          (bind _returnvalue_5 (Audio|SpawnSoundatLocation "/Game/SFX/Metasounds/MS_BasicSoundNoVariation.MS_BasicSoundNoVariation" (Transformation|GetActorLocation) "0, 0, 0" 0.5 1.0 0.0 "/Game/SFX/Attenuation/AS_Large.AS_Large" 0))
          (Class|AudioComponent|SetWaveParameter _returnvalue_5 "Sound" "/Game/SFX/WaveAssets/Magic/Laser.Laser"))
        (:then_2
          (if _returnvalue_3
            (Utilities|FlowControl|Sequence
              (:then_0
                (bind _returnvalue_6 (Audio|SpawnSoundatLocation "/Game/SFX/WaveAssets/Impacts/LaserImpact.LaserImpact" (.location _outhit) "0, 0, 0" 0.5 1.0 0.0 "/Game/SFX/Attenuation/AS_AttenuationMedium.AS_AttenuationMedium" 0))
                (Class|AudioComponent|SetWaveParameter _returnvalue_6 "Sound" "/Game/SFX/WaveAssets/Magic/Laser.Laser"))
              (:then_1
                (Utilities|IsValid (Actor|GetComponentbyClass (.hitactor _outhit) "/Game/Util/FunctionalComponents/BPC_Health.BPC_Health_C")
                  (:Is%20Valid
                    (Utilities|FlowControl|Delay 0.1)
                    (Class|BPIHealth|TakeDamage(Message) (Actor|GetComponentbyClass (.hitactor _outhit) "/Game/Util/FunctionalComponents/BPC_Health.BPC_Health_C") (Variables|Default|GetDamage) (Variables|Default|GetDamageType))))))))))
    (:then_2
      (Utilities|FlowControl|Delay 5.0)
      (Actor|DestroyActor))))

(event Collision|EventActorBeginOverlap
  (params (OtherActor :type Actor%20Object%20Reference)))

(event EventTick
  (params (DeltaSeconds :type Float%20%28single-precision%29)))

(fn ConstructionScript
  (|CallParentFunction))