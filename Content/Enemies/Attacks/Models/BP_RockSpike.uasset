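; Enemy attack actor for a rock spike that rises into place on spawn, with a randomly chosen mesh variant and stone-head enemy material.
; BeginPlay plays a MetaSound after a short random delay while a curve-driven Timeline lifts the mesh from its StartHeight offset.
; HitTrigger collision switches off once the rise completes.
; Retract reverses the Timeline and can destroy the actor after a delay.
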(event Custom|Retract
  (params (DestroyOnFinish :type Boolean))
  (Utilities|FlowControl|Sequence
    (:then_0
      (bind _c_rockspikerisecurve (Timeline|Timeline Reverse)
        (:Update
          (Transformation|SetRelativeLocation (Variables|Default|GetStaticMesh) (Math|Vector|MakeVector 0.0 0.0 (* (- 1.0 _c_rockspikerisecurve) (Variables|Default|GetStartHeight) -1.0)) false false)
          (if (>= (* (- 1.0 _c_rockspikerisecurve) (Variables|Default|GetStartHeight) -1.0) 0.0)
            (Collision|SetCollisionEnabled (Variables|Default|GetHitTrigger) "NoCollision")
            (Timeline|Timeline Stop)))))
    (:then_1
      (if DestroyOnFinish
        (Utilities|FlowControl|Delay 1.0)
        (Actor|DestroyActor)))))

(event EventBeginPlay
  (Utilities|FlowControl|Sequence
    (:then_0
      (if true
        (Utilities|FlowControl|Delay (Math|Random|RandomFloatinRange 0.0 0.3))
        (bind _returnvalue (Audio|SpawnSoundatLocation "/Game/SFX/Metasounds/MS_BasicVariation.MS_BasicVariation" (Transformation|GetActorLocation) "0, 0, 0" 1.0 1.0 0.0 0 0))
        (Class|AudioComponent|SetWaveParameter _returnvalue "Sound" "/Game/SFX/WaveAssets/Impacts/RockSpikes.RockSpikes")))
    (:then_1
      (bind _c_rockspikerisecurve (Timeline|Timeline Play)
        (:Update
          (Transformation|SetRelativeLocation (Variables|Default|GetStaticMesh) (Math|Vector|MakeVector 0.0 0.0 (* (- 1.0 _c_rockspikerisecurve) (Variables|Default|GetStartHeight) -1.0)) false false)
          (if (>= (* (- 1.0 _c_rockspikerisecurve) (Variables|Default|GetStartHeight) -1.0) 0.0)
            (Collision|SetCollisionEnabled (Variables|Default|GetHitTrigger) "NoCollision")
            (Timeline|Timeline Stop)))))))

(fn ConstructionScript
  (bind _staticmesh (Variables|Default|GetStaticMesh))
  (Components|StaticMesh|SetStaticMesh _staticmesh (.OutItem (Utilities|Array|Random (Utilities|Array|MakeArray "/Game/Enemies/Attacks/Models/StoneSpikes_Cube.StoneSpikes_Cube" "/Game/Enemies/Attacks/Models/StoneSpikes_Cube_001.StoneSpikes_Cube_001" "/Game/Enemies/Attacks/Models/StoneSpikes_Cube_002.StoneSpikes_Cube_002"))))
  (Rendering|Material|SetMaterial _staticmesh 0 "/Game/Enemies/Models/StoneHead/Textures/M_Enemy_StoneHead.M_Enemy_StoneHead"))