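; Enemy attack actor that deals a single instance of damage in front of itself as soon as it begins play.
; On BeginPlay it sphere-traces along its forward vector using its Range and Radius, ignoring the Enemy reference.
; If the hit actor has a BPC_Health component, it sends that component a TakeDamage message with the attack's damage amount and type.
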(event EventBeginPlay
  (bind _returnvalue (Transformation|GetActorLocation))
  (bind (_outhit _returnvalue_2) (Collision|SphereTraceByChannel _returnvalue (+ _returnvalue (* (Transformation|GetActorForwardVector) (Variables|Default|GetRange))) (Variables|Default|GetRadius) "TraceTypeQuery3" false (Utilities|Array|MakeArray (Variables|Default|GetEnemy)) "None"))
  (if _returnvalue_2
    (Utilities|IsValid (Actor|GetComponentbyClass (.hitactor _outhit) "/Game/Util/FunctionalComponents/BPC_Health.BPC_Health_C")
      (:Is%20Valid
        (Class|BPIHealth|TakeDamage(Message) (Actor|GetComponentbyClass (.hitactor _outhit) "/Game/Util/FunctionalComponents/BPC_Health.BPC_Health_C") (Variables|Default|GetDamage) (Variables|Default|GetDamageType))))))

(fn ConstructionScript)