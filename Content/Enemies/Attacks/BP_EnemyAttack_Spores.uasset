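; BP_EnemyAttack_Spores is an enemy attack that creates a spore hazard which poisons the player on contact.
; While active, its sphere overlap applies a timed poison status effect to the player.
; The first successful hit or the end of its lifetime deactivates it and sets the Niagara spawn rate to zero, with no explicit destroy.
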(event OnComponentBeginOverlap(Sphere)
  (params (OverlappedComponent :type Primitive%20Component%20Object%20Reference) (OtherActor :type Actor%20Object%20Reference) (OtherComp :type Primitive%20Component%20Object%20Reference) (OtherBodyIndex :type Integer) (bFromSweep :type Boolean) (SweepResult :type Hit%20Result%20Structure%20%28by%20ref%29))
  (if (Variables|Default|GetActive)
    (bind _asbp_player (Utilities|Casting|CastToBP_Player OtherActor))
    (CallFunction|ApplyStatusEffect "/Game/Util/StatusEffects/BPC_StatusEffect_Poison.BPC_StatusEffect_Poison_C" _asbp_player 1e+01)
    (Variables|Default|SetActive false)
    (Effects|Components|ParticleSystem|SetFloatParameter (Variables|Default|GetNiagara) "SpawnRateMultiplier" 0.0)))

(event EventBeginPlay
  (Utilities|FlowControl|Delay (Variables|Default|GetLifetime))
  (Variables|Default|SetActive false)
  (Effects|Components|ParticleSystem|SetFloatParameter (Variables|Default|GetNiagara) "SpawnRateMultiplier" 0.0))

(fn ConstructionScript
  (|CallParentFunction))